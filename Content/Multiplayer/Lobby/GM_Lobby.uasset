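; Lobby game mode that registers players as they join a multiplayer lobby and keeps their lists in sync.
; On PostLogin it stores each PC_Lobby controller, assigns an incrementing ID, collects its PlayerInfo and, after a short delay, pushes the full list to every connected controller.
; Tick copies the connected player count to OnlineGameInstance and prints it on screen every frame.
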(event EventBeginPlay)

(event EventTick
  (params (DeltaSeconds :type Float%20%28single-precision%29))
  (bind _output_get (Variables|Default|SetTotalPlayers (Utilities|Array|Length (Variables|Default|GetConnectedPlayers))))
  (Development|PrintString (Utilities|String|ToString(Integer) _output_get))
  (bind _asonline_game_instance (Utilities|Casting|CastToOnlineGameInstance (Game|GetGameInstance)))
  (Variables|/Game/Multiplayer/OnlineGameInstance.OnlineGameInstance_C|SetTotalPlayers _asonline_game_instance (Variables|Default|GetTotalPlayers)))

(event EventPostLogin
  (params (NewPlayer :type Player%20Controller%20Object%20Reference))
  (bind _aspc_lobby (Utilities|Casting|CastToPC_Lobby NewPlayer))
  (Utilities|Array|Add (Variables|Default|GetConnectedPlayers) _aspc_lobby)
  (Variables|/Game/Multiplayer/Lobby/PC_Lobby.PC_Lobby_C|SetPlayerID _aspc_lobby (Variables|Default|GetNextPlayerID))
  (Variables|Default|SetNextPlayerID (+ (Variables|Default|GetNextPlayerID) 1))
  (Utilities|Array|Add (Variables|Default|GetConnectedPlayerInfo) (Variables|/Game/Multiplayer/Lobby/PC_Lobby.PC_Lobby_C|GetPlayerInfo _aspc_lobby))
  (Utilities|FlowControl|Delay 0.2)
  (for _array_element (Variables|Default|GetConnectedPlayers)
    (Default|UpdatePlayerList _array_element (Variables|Default|GetConnectedPlayerInfo))))

(fn ConstructionScript)