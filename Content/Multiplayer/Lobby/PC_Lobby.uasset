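; Lobby player controller for multiplayer: shows host or client menus by authority, spawns a preview truck pawn and stores player choices in OnlineGameInstance.
; Team and Vehicle RepNotifies recolour the possessed vehicle, while player list updates feed only the host widget.
; StartGame notifies GM_Lobby, then opens SpaceArena as a listen server after a delay.
; TransitionAllButServer sends remote clients to TransitionMap, carrying the session ID as a URL option.
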(event Custom|StartGame
  (params (CurrentMap :type String))
  (CallFunction|ShowLoadingScreen)
  (bind _asgm_lobby (Utilities|Casting|CastToGM_Lobby (Game|GetGameMode)))
  (Default|HostPressedStart _asgm_lobby)
  (Utilities|FlowControl|Delay 1.0)
  (Game|OpenLevel(byObjectReference) "/Game/Levels/SpaceArena.SpaceArena" true "listen"))

(event Custom|UpdatePlayerList
  (params (PlayerInfo :type Array%20of%20Player%20Info%20Struct%20Structures))
  (Variables|Default|SetConnectedPlayerInfo PlayerInfo)
  (Networking|SwitchHasAuthority
    (:Authority
      (bind _asui_lobby_host_screen (Utilities|Casting|CastToUI_LobbyHostScreen (Variables|Default|GetLobbyWidget)))
      (Default|UpdatePlayerList _asui_lobby_host_screen (Variables|Default|GetConnectedPlayerInfo)))))

(event Custom|ChangeCharacter
  (params (NewVehicle :type BP%20Wheeled%20Vehicle%20Base%20Class%20Reference))
  (bind _returnvalue (Pawn|GetControlledPawn))
  (Variables|Default|SetSpawnTransform (Transformation|GetActorTransform _returnvalue))
  (Actor|DestroyActor _returnvalue)
  (bind _returnvalue_2 (Game|SpawnActorfromClass NewVehicle (Math|Transform|MakeTransform (Math|Vector|MakeVector (.x (.location (Variables|Default|GetSpawnTransform))) (.y (.location (Variables|Default|GetSpawnTransform))) 1.8e+02) (.rotation (Variables|Default|GetSpawnTransform)) (.scale (Variables|Default|GetSpawnTransform))) "Undefined" 0 0))
  (bind _output_get (Variables|Default|SetVehicle _returnvalue_2))
  (Pawn|Possess _output_get))

(event Custom|SetVehicleClass
  (params (ChosenVehicle :type BP%20Wheeled%20Vehicle%20Base%20Class%20Reference))
  (bind _asonline_game_instance (Utilities|Casting|CastToOnlineGameInstance (Game|GetGameInstance)))
  (Variables|/Game/Multiplayer/OnlineGameInstance.OnlineGameInstance_C|SetChosenVehicle _asonline_game_instance ChosenVehicle))

(event Custom|CreateMenus
  (Networking|SwitchHasAuthority
    (:Authority
      (bind _returnvalue (UserInterface|CreateWidget "/Game/Multiplayer/Lobby/UI_LobbyHostScreen.UI_LobbyHostScreen_C"))
      (bind _output_get (Variables|Default|SetLobbyWidget _returnvalue))
      (UserInterface|Viewport|AddtoViewport _output_get 0))
    (:Remote
      (bind _returnvalue_2 (UserInterface|CreateWidget "/Game/Multiplayer/Lobby/UI_LobbyClientScreen.UI_LobbyClientScreen_C"))
      (bind _output_get_2 (Variables|Default|SetLobbyWidget _returnvalue_2))
      (UserInterface|Viewport|AddtoViewport _output_get_2 0))))

(event Custom|ShowLoadingScreen
  (bind _returnvalue (UserInterface|CreateWidget "/Game/Blueprints/UI/UI_Loading.UI_Loading_C" self))
  (UserInterface|Viewport|AddtoViewport _returnvalue 0))

(event Custom|SR_SetTeam
  (params (team :type Integer))
  (Variables|Default|SetTeam team))

(event Custom|TransitionAllButServer
  (Networking|SwitchHasAuthority
    (:Remote
      (bind _asonline_game_instance (Utilities|Casting|CastToOnlineGameInstance (Game|GetGameInstance)))
      (Development|PrintString (Variables|/Game/Multiplayer/OnlineGameInstance.OnlineGameInstance_C|GetSessionID _asonline_game_instance))
      (Game|OpenLevel(byObjectReference) "/Game/Levels/TransitionMap.TransitionMap" true (Utilities|String|Append "?SessionID=" (Variables|/Game/Multiplayer/OnlineGameInstance.OnlineGameInstance_C|GetSessionID _asonline_game_instance))))))

(event EventBeginPlay
  (if (Pawn|IsLocalController)
    (CallFunction|CreateMenus)
    (Utilities|FlowControl|Delay 0.2)
    (bind _asonline_game_instance (Utilities|Casting|CastToOnlineGameInstance (Game|GetGameInstance)))
    (bind _output_get (Variables|/Game/Multiplayer/OnlineGameInstance.OnlineGameInstance_C|SetCurrentPlayer _asonline_game_instance (Variables|Default|GetPlayerID)))
    (CallFunction|SRSetTeam _output_get)
    (CallFunction|ChangeCharacter "/Game/Blueprints/Pawns/BPW_Truck.BPW_Truck_C")))

(event EventTick
  (params (DeltaSeconds :type Float%20%28single-precision%29)))

(fn ConstructionScript)

(fn OnRepTeam
  (if (Utilities|IsValid (Variables|Default|GetVehicle))
    (Default|SetColour (Variables|Default|GetVehicle) (Variables|Default|GetTeam))))

(fn OnRepVehicle
  (Default|SetColour (Variables|Default|GetVehicle) (Variables|Default|GetTeam)))