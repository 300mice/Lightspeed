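; Actor that holds per-team trail cubes as instanced meshes, one instanced component each for blue, red, yellow and purple.
; SpawnCube adds an instance at a given transform to the component matching the team index, with blue as the fallback.
; DestroyTrail clears all instances from the chosen team's component, so each team's trail is wiped independently.
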(event Custom|DestroyTrail
  (params (inputTeam :type Integer))
  (switch int inputTeam
    (:Default
      (Components|InstancedStaticMesh|ClearInstances (Variables|Default|GetBlueTrail) :!label _label))
    (:0
      (goto _label))
    (:1
      (Components|InstancedStaticMesh|ClearInstances (Variables|Default|GetRedTrail)))
    (:2
      (Components|InstancedStaticMesh|ClearInstances (Variables|Default|GetYellowTrail)))
    (:3
      (Components|InstancedStaticMesh|ClearInstances (Variables|Default|GetPurpleTrail)))))

(event EventBeginPlay)

(event Collision|EventActorBeginOverlap
  (params (OtherActor :type Actor%20Object%20Reference)))

(event EventTick
  (params (DeltaSeconds :type Float%20%28single-precision%29)))

(fn ConstructionScript)

(fn SpawnCube
  (params (Transform :type Transform) (Team :type Integer))
  (switch int Team
    (:Default
      (Components|InstancedStaticMesh|AddInstance (Variables|Default|GetBlueTrail) Transform :!label _label))
    (:0
      (goto _label))
    (:1
      (Components|InstancedStaticMesh|AddInstance (Variables|Default|GetRedTrail) Transform))
    (:2
      (Components|InstancedStaticMesh|AddInstance (Variables|Default|GetYellowTrail) Transform))
    (:3
      (Components|InstancedStaticMesh|AddInstance (Variables|Default|GetPurpleTrail) Transform))))