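; Game mode for a local multiplayer race that sets up players, menu input and truck spawning.
; On BeginPlay it creates a local player for each PlayerStart, matched by numeric tag, possessing a BP_PlayerInput pawn there, then shows the menu widget.
; DisplayCharacterSelect adds a per-player selection panel to that menu and links it to the input pawn.
; SpawnPlayer spawns a BP_BVTruck at the input pawn's transform and hands possession to it.
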(event EventBeginPlay
  (CallFunction|GetPlayerStartPoints)
  (CallFunction|SpawnInputRecievers)
  (bind _returnvalue (UserInterface|CreateWidget "/Game/Blueprints/UI/UI_Menu.UI_Menu_C"))
  (bind _output_get (Variables|Default|SetMenuWidgetRef _returnvalue))
  (UserInterface|Viewport|AddtoViewport _output_get 0))

(event EventTick
  (params (DeltaSeconds :type Float%20%28single-precision%29)))

(fn ConstructionScript)

(fn GetPlayerStartPoints
  (bind _outactors (Actor|GetAllActorsOfClass "/Script/Engine.PlayerStart"))
  (Variables|Default|SetPlayerStartArray _outactors))

(fn SpawnInputRecievers
  (for (_ _array_index) (Variables|Default|GetPlayerStartArray)
    (LocalVariables|SetIndex _array_index)
    (for _array_element (Variables|Default|GetPlayerStartArray)
      (if (== (CallFunction|NametoInt _array_element) (LocalVariables|GetIndex))
        (Class|GameplayStatics|CreatePlayer -1)
        (bind _returnvalue (Game|SpawnActorfromClass "/Game/Blueprints/GameBP/BP_PlayerInput.BP_PlayerInput_C" (Transformation|GetActorTransform (Utilities|Array|Get(acopy) (Variables|Default|GetPlayerStartArray) (LocalVariables|GetIndex))) "Undefined" 0 (LocalVariables|GetIndex) 0))
        (Utilities|Array|AddUnique (Variables|Default|GetPlayerInputRecieverArray) _returnvalue)
        (Pawn|Possess (Game|GetPlayerController (LocalVariables|GetIndex)) _returnvalue)
        (Utilities|Array|AddUnique (Variables|Default|GetPlayerControllerArray) (Game|GetPlayerController (LocalVariables|GetIndex)))))))

(fn NametoInt
  (params (PlayerStart :type Player%20Start%20Object%20Reference))
  (return (Math|Conversions|ToInteger(Byte) (Utilities|String|ToString(Name) (Variables|/Script/Engine.PlayerStart|GetPlayerStartTag PlayerStart)))))

(fn DisplayCharacterSelect
  (params (CurrentPlayerIndex :type Integer))
  (bind _characterselect (Default|AddCharacterSelect (Variables|Default|GetMenuWidgetRef) CurrentPlayerIndex))
  (Variables|/Game/Blueprints/GameBP/BP_PlayerInput.BP_PlayerInput_C|SetCharacterMenuRef (Utilities|Array|Get(acopy) (Variables|Default|GetPlayerInputRecieverArray) CurrentPlayerIndex) _characterselect)
  (return false))

(fn SpawnPlayer
  (params (CurrentPlayerIndex :type Integer) (InputReciever :type BP%20Player%20Input%20Object%20Reference))
  (bind _returnvalue (Game|SpawnActorfromClass "/Game/Blueprints/Vehicle/BP_BVTruck.BP_BVTruck_C" (Transformation|GetActorTransform InputReciever) "Undefined" 0 CurrentPlayerIndex 0))
  (Pawn|Possess (Game|GetPlayerController CurrentPlayerIndex) _returnvalue)
  (return false))