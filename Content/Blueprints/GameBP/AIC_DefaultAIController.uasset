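; AI controller for a BP_BaseVehicle that starts the BT_DefaultAI behavior tree on BeginPlay and calls TronForward every Tick.
; Helper functions sphere-trace ahead while ignoring Floors, compare left and right hit distances, and yaw the vehicle by fixed steps.
; Both turn functions are identical, following LeftAngle and ignoring their ChosenAngle input.
; The vehicle cast and "Floor" tag lookup are disconnected, so this graph never sets those variables.
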(event EventBeginPlay
  (AI|RunBehaviorTree "/Game/Blueprints/AI/BT_DefaultAI.BT_DefaultAI"))

(event EventTick
  (params (DeltaSeconds :type Float%20%28single-precision%29))
  (CallFunction|TronForward self))

(fn ConstructionScript)

(fn CollisionLineTrace
  (params (Target :type Scene%20Component%20Object%20Reference) (Distance :type Float%20%28single-precision%29))
  (bind _returnvalue (Transformation|GetWorldLocation Target))
  (bind (_outhit _returnvalue_2) (Collision|SphereTraceByChannel _returnvalue (+ (* (Math|Vector|GetForwardVector Target) Distance) _returnvalue) 2e+02 "TraceTypeQuery1" false (Variables|Default|GetFloors) "ForOneFrame"))
  (return _outhit _returnvalue_2))

(fn AdjustTurnAngleRight
  (params (ChosenAngle :type Float%20%28single-precision%29))
  (if (Variables|Default|GetbLeftAngle)
    (Class|Actor|AddActorWorldRotation (Variables|Default|GetAs%20BP%20Base%20Vehicle) "0,-0.700000, 0")
    (else
      (Class|Actor|AddActorWorldRotation (Variables|Default|GetAs%20BP%20Base%20Vehicle) "0,0.700000, 0"))))

(fn AdjustTurnAngleLeft
  (params (ChosenAngle :type Float%20%28single-precision%29))
  (if (Variables|Default|GetbLeftAngle)
    (Class|Actor|AddActorWorldRotation (Variables|Default|GetAs%20BP%20Base%20Vehicle) "0,-0.700000, 0")
    (else
      (Class|Actor|AddActorWorldRotation (Variables|Default|GetAs%20BP%20Base%20Vehicle) "0,0.700000, 0"))))

(fn GetLargerDistance
  (bind _as_bp_base_vehicle (Variables|Default|GetAs%20BP%20Base%20Vehicle))
  (if (> (Math|Float|Absolute(Float) (Math|Vector|VectorLength (- (.impactpoint (Variables|Angle|GetLeftHit)) (Transformation|GetWorldLocation (Variables|/Game/Blueprints/Vehicle/BP_BaseVehicle.BP_BaseVehicle_C|GetLeftDetection _as_bp_base_vehicle))))) (Math|Float|Absolute(Float) (Math|Vector|VectorLength (- (.impactpoint (Variables|Angle|GetRightHit)) (Transformation|GetWorldLocation (Variables|/Game/Blueprints/Vehicle/BP_BaseVehicle.BP_BaseVehicle_C|GetRightDetection _as_bp_base_vehicle))))))
    (return false)
    (else
      (return true))))