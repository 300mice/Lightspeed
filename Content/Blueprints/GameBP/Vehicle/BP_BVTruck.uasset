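; BP_BVTruck is a truck vehicle Blueprint with a wall-dropping ability.
; Pressing the Ability input spawns a BP_WallAbility 200 units behind the truck, matching its rotation.
; Any actor overlap runs the parent handler and then destroys the truck itself, with no filter on the other actor.
; Tick and the construction script only call their parent versions.
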(event EventBeginPlay
  (|CallParentFunction) ; This node is disabled and will not be called.\nDrag off pins to build functionality.
)

(event Collision|EventActorBeginOverlap
  (params (OtherActor :type Actor%20Object%20Reference))
  (|CallParentFunction OtherActor)
  (Actor|DestroyActor))

(event EventTick
  (params (DeltaSeconds :type Float%20%28single-precision%29))
  (|CallParentFunction DeltaSeconds))

(event Input|ActionEvents|InputActionAbility
  (params (Key :type Key%20Structure :default "None"))
  (bind _returnvalue (Transformation|GetActorTransform))
  (:Pressed
    (Game|SpawnActorfromClass "/Game/Blueprints/Abilities/BP_WallAbility.BP_WallAbility_C" (Math|Transform|MakeTransform (+ (.location _returnvalue) (* (Transformation|GetActorForwardVector) -2e+02)) (.rotation _returnvalue) "1,1,1") "Undefined" 0 0)))

(fn ConstructionScript
  (|CallParentFunction))