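; PC_VehicleController is a player controller that drives a Tron-style, continuously moving vehicle pawn with mouse steering.
; While the Moving flag is set through SetMoving, Tick calls TronForward and MouseSteeringControls.
; Steering converts the mouse's horizontal viewport position into a rounded, center-zero offset, added as yaw each frame without delta-time scaling.
; ContinuousTronMovement applies forced forward movement input, but Tick does not call it by that name.
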(event EventBeginPlay)

(event EventTick
  (params (DeltaSeconds :type Float%20%28single-precision%29))
  (if (Variables|Default|GetbMoving)
    (CallFunction|TronForward self)
    (CallFunction|MouseSteeringControls)))

(event EventSetMoving
  (params (bMoving :type Boolean))
  (Variables|Default|SetbMoving bMoving))

(fn ConstructionScript)

(fn MouseSteeringControls
  ;[1 1 1] Get Viewport size and divide mouse position by half so that center = 0, left = -0.5, right = 0.5
  (bind _returnvalue (Class|WidgetLayoutLibrary|GetMousePositiononViewport))
  (bind _roundedfloat (CallFunction|RoundtoDecimal (/ (* (.x _returnvalue) (Class|WidgetLayoutLibrary|GetViewportScale)) (.x (Viewport|GetViewportSize))) 1e+01))
  (Class|Actor|AddActorWorldRotation (Pawn|GetControlledPawn) (Math|Rotator|MakeRotator 0.0 0.0 (- _roundedfloat 0.5))))

(fn ContinuousTronMovement
  (bind _returnvalue (Pawn|GetControlledPawn))
  (Pawn|Input|AddMovementInput _returnvalue (Transformation|GetActorForwardVector _returnvalue) 1.0 true))