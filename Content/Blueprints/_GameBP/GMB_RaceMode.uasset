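; Race game mode, apparently unfinished, that tracks joining players and provides helpers to spawn them at PlayerStart points.
; PostLogin collects vehicle controllers, and Tick compares their count to TotalPlayers before a delay and empty loop.
; SpawnPlayers possesses a test character at successive starts, ignoring its Vehicle input.
; A helper spawns player or behavior-tree AI vehicles, but its callers, TotalPlayers initialization and several function bodies are disconnected.
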(event Custom|SpawnPlayers
  (params (PlayerController :type Player%20Controller%20Object%20Reference) (Vehicle :type BP%20Base%20Vehicle%20Class%20Reference))
  (bind _returnvalue (Pawn|GetControlledPawn PlayerController))
  (Utilities|IsValid _returnvalue
    (:Is%20Valid
      (Actor|DestroyActor _returnvalue))
    (:Is%20Not%20Valid
      _))
  (bind _returnvalue_2 (Game|SpawnActorfromClass "/Game/Blueprints/Vehicle/BP_BaseCharacterClassTest.BP_BaseCharacterClassTest_C" (Transformation|GetActorTransform (Utilities|Array|Get(acopy) (Variables|Default|GetPlayerStartArray) (Variables|Default|GetPlayerStartIndex))) "Undefined" PlayerController 0))
  (Pawn|Possess PlayerController _returnvalue_2)
  (Variables|Default|SetPlayerStartIndex (+ (Variables|Default|GetPlayerStartIndex) 1)))

(event EventBeginPlay
  (CallFunction|GetPlayerStartPoints))

(event EventTick
  (params (DeltaSeconds :type Float%20%28single-precision%29))
  (if (== (Variables|Default|GetPlayersReady) (Variables|Default|GetTotalPlayers))
    (if (not (Variables|Default|GetStartedGame))
      (Utilities|FlowControl|DoOnce false
        (:Completed
          (Utilities|FlowControl|Delay 5.0)
          (for _array_element (Variables|Default|GetConnectedPlayers)
            _))))
    (else
      (Development|PrintString "Hello"))))

(event EventPostLogin
  (params (NewPlayer :type Player%20Controller%20Object%20Reference))
  (bind _aspc_vehicle_controller (Utilities|Casting|CastToPC_VehicleController NewPlayer))
  (Utilities|Array|Add (Variables|Default|GetConnectedPlayers) _aspc_vehicle_controller)
  (Math|Integer|IncrementInt (Variables|Default|GetPlayersReady)))

(fn ConstructionScript)

(fn GetPlayerStartPoints
  (bind _outactors (Actor|GetAllActorsOfClass "/Script/Engine.PlayerStart"))
  (Variables|Default|SetPlayerStartArray _outactors))

(fn SpawnInputRecievers)

(fn NametoInt
  (params (PlayerStart :type Player%20Start%20Object%20Reference))
  (return (Math|Conversions|ToInteger(Byte) (Utilities|String|ToString(Name) (Variables|/Script/Engine.PlayerStart|GetPlayerStartTag PlayerStart)))))

(fn SpawnVehicleOfChosenType
  (params (Dimension%201 :type Integer) (AI :type Boolean) (PawnClass :type Pawn%20Class%20Reference))
  (bind _playerstartarray (Variables|Default|GetPlayerStartArray))
  (bind _output (Utilities|Array|Get(acopy) _playerstartarray Dimension%201))
  (bind _returnvalue (Transformation|GetActorTransform _output))
  (if AI
    (AI|SpawnAIFromClass PawnClass "/Game/Blueprints/AI/BT_DefaultAI.BT_DefaultAI" (.location _returnvalue) (.rotation _returnvalue) false 0)
    (Development|PrintString (Utilities|String|ToString(Vector) (.location _returnvalue)))
    (return 0)
    (else
      (bind _returnvalue_2 (Game|SpawnActorfromClass PawnClass (Transformation|GetActorTransform (Utilities|Array|Get(acopy) (Variables|Default|GetPlayerStartArray))) "Undefined" (Game|GetPlayerController Dimension%201) 0))
      (Development|PrintString "ME")
      (return _returnvalue_2))))

(fn SpawnDefaultPawnfor
  (params (NewPlayer :type Controller%20Object%20Reference) (StartSpot :type Actor%20Object%20Reference)))

(fn DisplayCharacterSelect
  (params (CurrentPlayerIndex :type Integer))
  (bind _characterselect (Default|AddCharacterSelect (Variables|Default|GetMenuWidgetRef) CurrentPlayerIndex))
  (Variables|/Game/Blueprints/_GameBP/BP_PlayerInput.BP_PlayerInput_C|SetCharacterMenuRef (Utilities|Array|Get(acopy) (Variables|Default|GetPlayerInputRecieverArray) CurrentPlayerIndex) _characterselect)
  (return false))

(fn GetFloor
  (return (Variables|Default|GetFlooring)))

(fn SpawnPlayer
  (params (CurrentPlayerIndex :type Integer) (InputReciever :type BP%20Player%20Input%20Object%20Reference)))