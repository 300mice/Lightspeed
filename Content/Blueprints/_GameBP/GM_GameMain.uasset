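; Game mode for a multiplayer car game that tracks connected controllers, places players at level PlayerStarts and advances rounds.
; PostLogin collects vehicle controllers; Spawning replaces a player's pawn with the given vehicle at the next start, while StartUp restarts everyone across successive starts.
; RoundUp increments the GameState round and decrements the alive count for dead players.
; ReadyToStartMatch always returns false; the round timer and AI-truck slot filling are disconnected.
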(event Custom|GetPlayerStartPoints
  ;[1 1 1] Creates an array of all player start locations
  (bind _outactors (Actor|GetAllActorsOfClass "/Script/Engine.PlayerStart"))
  (Variables|Default|SetPlayerStartPoints _outactors))

(event Custom|RoundUp
  ;[1 1 1] Begin Play
  (bind _asgs_car_game (Utilities|Casting|CastToGS_CarGame (Game|GetGameState)))
  (Default|IncreaseRound _asgs_car_game)
  (for _array_element (Variables|Default|GetConnectedPlayers)
    (bind _asps_player_state (Utilities|Casting|CastToPS_PlayerState (Variables|/Script/Engine.Controller|GetPlayerState _array_element)))
    (if (Variables|/Game/Blueprints/PS_PlayerState.PS_PlayerState_C|GetisDead? _asps_player_state)
      (Math|Integer|DecrementInt (Variables|Default|GetPlayersAlive)
        (:%20%20
          (Development|PrintString (Utilities|String|ToString(Integer) (Variables|Default|GetPlayersAlive))))))))

(event Custom|StartUp
  (for _array_element (Variables|Default|GetConnectedPlayers)
    (Class|GameModeBase|RestartPlayeratPlayerStart _array_element (Utilities|Array|Get(acopy) (Variables|Default|GetPlayerStartPoints) (Variables|Default|GetPlayer%20Start%20Index)))
    (Variables|Default|SetPlayer%20Start%20Index (+ (Variables|Default|GetPlayer%20Start%20Index) 1))))

(event Custom|Spawning
  (params (vehicle :type BP%20Base%20Character%20Class%20Test%20Class%20Reference) (player%20controller :type Player%20Controller%20Object%20Reference))
  (bind _returnvalue (Pawn|GetControlledPawn player%20controller))
  ;[1 1 1] Spawns each player as their chosen vehicle and assigns them to a player start position
  (Utilities|IsValid _returnvalue
    (:Is%20Valid
      (Actor|DestroyActor _returnvalue))
    (:Is%20Not%20Valid
      _))
  (bind _returnvalue_2 (Game|SpawnActorfromClass vehicle (Transformation|GetActorTransform (Utilities|Array|Get(acopy) (Variables|Default|GetPlayerStartPoints) (Variables|Default|GetPlayer%20Start%20Index))) "Undefined" player%20controller 0))
  (Pawn|Possess player%20controller _returnvalue_2)
  (Variables|Default|SetPlayer%20Start%20Index (+ (Variables|Default|GetPlayer%20Start%20Index) 1)))

(event EventBeginPlay
  ;[1 1 1] Begin Play
  (CallFunction|GetPlayerStartPoints))

(event EventHandleStartingNewPlayer
  (params (NewPlayer :type Player%20Controller%20Object%20Reference)))

(event EventPostLogin
  (params (NewPlayer :type Player%20Controller%20Object%20Reference))
  ;[1 1 1] When a player logins into the game, add them to an array of connected player controllers
  (bind _aspc_vehicle_controller (Utilities|Casting|CastToPC_VehicleController NewPlayer))
  (Utilities|Array|Add (Variables|Default|GetConnectedPlayers) _aspc_vehicle_controller)
  (Math|Integer|IncrementInt (Variables|Default|GetNumPlayersConnected)))

(event EventTick
  (params (DeltaSeconds :type Float%20%28single-precision%29)))

(fn ConstructionScript)

(fn ReadytoStartMatch
  (return false))