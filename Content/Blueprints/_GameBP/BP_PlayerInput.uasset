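; BP_PlayerInput receives a player's StartGame input and forwards join requests to the game mode.
; On press, AddPlayer checks whether its character menu reference is valid.
; With a valid menu, it asks the game mode to spawn the player, passing the player index and itself as input receiver.
; Otherwise, it asks the game mode to display character select for that player index.
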(event Custom|AddPlayer
  (Utilities|IsValid (Variables|Default|GetCharacterMenuRef)
    (:Is%20Valid
      (Class|BPIGameMode|SpawnPlayer(Message) (Game|GetGameMode) (Variables|Default|GetPlayerIndex) self))
    (:Is%20Not%20Valid
      (Class|BPIGameMode|DisplayCharacterSelect(Message) (Game|GetGameMode) (Variables|Default|GetPlayerIndex)))))

(event EventBeginPlay)

(event Collision|EventActorBeginOverlap
  (params (OtherActor :type Actor%20Object%20Reference)))

(event EventTick
  (params (DeltaSeconds :type Float%20%28single-precision%29)))

(event Input|ActionEvents|InputActionStartGame
  (params (Key :type Key%20Structure))
  (:Pressed
    (CallFunction|AddPlayer)))

(event Input|ActionEvents|InputActionMenuLeft
  (params (Key :type Key%20Structure)))

(event Input|ActionEvents|InputActionMenuRight
  (params (Key :type Key%20Structure)))

(fn ConstructionScript)