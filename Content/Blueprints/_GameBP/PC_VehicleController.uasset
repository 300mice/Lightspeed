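; Player controller for the vehicle race mode that requests the player's chosen vehicle and drives its input.
; BeginPlay reads the vehicle choice from OnlineGameInstance and caches the race mode and possessed BP_BaseVehicle.
; StartGame calls SendToServer, which has GMB_RaceMode spawn the player, while Tick calls the vehicle's mouse input handler.
; Viewport-relative mouse steering and Tron-style constant forward movement functions remain, but nothing live here calls them.
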(event Custom|GetVehicleClass
  (bind _asonline_game_instance (Utilities|Casting|CastToOnlineGameInstance (Game|GetGameInstance)))
  (Variables|Default|SetChosen%20Vehicle (Variables|/Game/Multiplayer/OnlineGameInstance.OnlineGameInstance_C|GetChosenVehicle _asonline_game_instance)))

(event Custom|SendToServer
  (bind _asgmb_race_mode (Utilities|Casting|CastToGMB_RaceMode (Game|GetGameMode)))
  (Default|SpawnPlayers _asgmb_race_mode self (Variables|Default|GetChosen%20Vehicle))
  (Variables|Default|SetbMoving true))

(event Custom|StartGame
  (CallFunction|SendtoServer))

(event EventBeginPlay
  (CallFunction|GetVehicleClass)
  (bind _asgmb_race_mode (Utilities|Casting|CastToGMB_RaceMode (Game|GetGameMode)))
  (Variables|Default|SetAs%20GMB%20Race%20Mode _asgmb_race_mode)
  (bind _asbp_base_vehicle (Utilities|Casting|CastToBP_BaseVehicle (Pawn|GetControlledPawn)))
  (Variables|Default|SetBaseVehicle _asbp_base_vehicle))

(event EventTick
  (params (DeltaSeconds :type Float%20%28single-precision%29))
  (Default|RecieveMouseInput (Variables|Default|GetBaseVehicle)))

(event EventSetMoving
  (params (bMoving :type Boolean))
  (Variables|Default|SetbMoving bMoving))

(fn ConstructionScript)

(fn MouseSteeringControls
  ;[1 1 1] Get Viewport size and divide mouse position by half so that center = 0, left = -0.5, right = 0.5
  (bind _returnvalue (Class|WidgetLayoutLibrary|GetMousePositiononViewport))
  (bind _roundedfloat (CallFunction|RoundtoDecimal (/ (* (.x _returnvalue) (Class|WidgetLayoutLibrary|GetViewportScale)) (.x (Viewport|GetViewportSize))) 1e+01))
  (Class|Actor|AddActorWorldRotation (Pawn|GetControlledPawn) (Math|Rotator|MakeRotator 0.0 0.0 (- _roundedfloat 0.5))))

(fn ContinuousTronMovement
  (bind _returnvalue (Pawn|GetControlledPawn))
  (Pawn|Input|AddMovementInput _returnvalue (Transformation|GetActorForwardVector _returnvalue) 1.0 true))