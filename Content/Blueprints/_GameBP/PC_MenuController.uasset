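; PC_MenuController is the menu player controller that handles the hand-off from an "insert coin" start screen to the main menu.
; On BeginPlay it creates the UI_InsertCoin widget, stores it and adds it to the viewport.
; An AnyKey press removes that widget, adds a new UI_MainMenu, sets Game and UI input mode and shows the mouse cursor.
; The key handler has no guard, so each press creates another main menu widget.
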(event EventBeginPlay
  (bind _returnvalue (UserInterface|CreateWidget "/Game/Blueprints/UI/UI_InsertCoin.UI_InsertCoin_C"))
  (bind _output_get (Variables|Default|SetStartUpUI _returnvalue))
  (UserInterface|Viewport|AddtoViewport _output_get 0))

(event EventTick
  (params (DeltaSeconds :type Float%20%28single-precision%29)))

(event Input|ActionEvents|InputActionAnyKey
  (params (Key :type Key%20Structure :default "None"))
  (:Pressed
    (Widget|RemovefromParent (Variables|Default|GetStartUpUI))
    (bind _returnvalue (UserInterface|CreateWidget "/Game/Multiplayer/UI_MainMenu.UI_MainMenu_C"))
    (UserInterface|Viewport|AddtoViewport _returnvalue 0)
    (Input|SetInputModeGameandUI self 0 "DoNotLock" true)
    (Variables|Default|SetbShowMouseCursor true)))

(fn ConstructionScript)