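; Transition player controller that automatically rejoins an online session whose ID is stored in the OnlineGameInstance.
; On BeginPlay it searches all server types with FindSessionsAdvanced and joins any result whose session ID matches the stored one, printing debug messages along the way.
; A failed search retries after a one-second delay through LoopServerFind, while a successful search with no match does not retry.
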(event Custom|LoopServerFind
  (bind _results (|FindSessionsAdvanced (Game|GetPlayerController 0) 0 false "AllServers" 0 false false false true)
    (:OnSuccess
      (for _array_element _results
        (Development|PrintString (Class|AdvancedSessionsLibrary|GetSessionIDasString _array_element) true true "(R=1.000000,G=0.000000,B=0.038177,A=1.000000)" 999.0)
        (if (== (Utilities|String|StringToName (Class|AdvancedSessionsLibrary|GetSessionIDasString _array_element)) (Variables|Default|GetSession%20ID))
          (|JoinSession (Game|GetPlayerController 0) _array_element
            (:then
              _)
            (:OnSuccess
              _))
          (Development|PrintString "Joining"))))
    (:OnFailure
      (Utilities|FlowControl|Delay 1.0)
      (Development|PrintString "FAILED TO FIND LOBBY" true true "(R=1.000000,G=0.155222,B=0.195027,A=1.000000)")
      (CallFunction|LoopServerFind))))

(event EventBeginPlay
  (bind _asonline_game_instance (Utilities|Casting|CastToOnlineGameInstance (Game|GetGameInstance)))
  (Variables|Default|SetSession%20ID (Variables|/Game/Multiplayer/OnlineGameInstance.OnlineGameInstance_C|GetSessionID _asonline_game_instance))
  (bind _results (|FindSessionsAdvanced (Game|GetPlayerController 0) 0 false "AllServers" 0 false false false true)
    (:OnSuccess
      (for _array_element _results
        (Development|PrintString (Class|AdvancedSessionsLibrary|GetSessionIDasString _array_element) true true "(R=1.000000,G=0.000000,B=0.038177,A=1.000000)" 999.0)
        (if (== (Utilities|String|StringToName (Class|AdvancedSessionsLibrary|GetSessionIDasString _array_element)) (Variables|Default|GetSession%20ID))
          (|JoinSession (Game|GetPlayerController 0) _array_element
            (:then
              _)
            (:OnSuccess
              _))
          (Development|PrintString "Joining"))))
    (:OnFailure
      (Utilities|FlowControl|Delay 1.0)
      (Development|PrintString "FAILED TO FIND LOBBY" true true "(R=1.000000,G=0.155222,B=0.195027,A=1.000000)")
      (CallFunction|LoopServerFind))))

(event EventTick
  (params (DeltaSeconds :type Float%20%28single-precision%29)))

(fn ConstructionScript)