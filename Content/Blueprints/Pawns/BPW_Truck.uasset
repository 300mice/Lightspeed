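; Truck pawn with a wall ability that spawns a team-coloured wall at its trail point.
; On BeginPlay it sets the ability cooldown time and, on authority only, its half-size extents.
; The Ability input calls SR_WallAbility, which, when not on cooldown, starts the cooldown, spawns BP_WallAbility and applies the team colour.
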(event Custom|SR_WallAbility
  (if (not (Variables|Default|GetbCooldown))
    (CallFunction|StartCooldown)
    (bind _returnvalue (Game|SpawnActorfromClass "/Game/Blueprints/Abilities/BP_WallAbility.BP_WallAbility_C" (Transformation|GetWorldTransform (Variables|Default|GetTrailPoint)) "Undefined" 0 0))
    (Default|SetColour _returnvalue (Variables|Default|GetTeam))))

(event EventBeginPlay
  (|CallParentFunction)
  (Variables|Default|SetCooldownTime 8.0)
  (Networking|SwitchHasAuthority
    (:Authority
      (Variables|Default|SetHalf%20Size "265.000000,155.000000,80.000000"))))

(event Collision|EventActorBeginOverlap
  (params (OtherActor :type Actor%20Object%20Reference))
  (|CallParentFunction OtherActor) ; This node is disabled and will not be called.\nDrag off pins to build functionality.
)

(event EventTick
  (params (DeltaSeconds :type Float%20%28single-precision%29))
  (|CallParentFunction DeltaSeconds) ; This node is disabled and will not be called.\nDrag off pins to build functionality.
)

(event Input|ActionEvents|InputActionAbility
  (params (Key :type Key%20Structure :default "None"))
  (:Pressed
    (CallFunction|SRWallAbility)))

(fn ConstructionScript
  (|CallParentFunction))