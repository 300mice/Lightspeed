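; Car pawn child Blueprint whose Ability input triggers a temporary invisibility cloak, named Decoy, with a cooldown.
; SR_Decoy starts the cooldown, toggles Client_Shadow around a timed delay and pauses an inherited timer meanwhile.
; Client_Shadow swaps mesh materials and plays or reverses a timeline that drives custom primitive data for the fade, delaying the restore.
; BeginPlay sets the cooldown and, on authority, the destructible actor class and half size.
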(event Custom|SR_Decoy
  (if (not (Variables|Default|GetbCooldown))
    (CallFunction|StartCooldown)
    (CallFunction|ClientShadow true)
    (Utilities|Time|PauseTimerbyHandle (Variables|Default|GetTimer))
    (Utilities|FlowControl|Delay 7.0)
    (CallFunction|ClientShadow false)
    (Utilities|Time|UnpauseTimerbyHandle (Variables|Default|GetTimer))))

(event Custom|Client_Shadow
  (params (On :type Boolean))
  (if On
    (CallFunction|UpdateMaterials (Variables|Default|GetInvisMaterial))
    (bind _time (Timeline|Transition Play)
      (:Update
        (Rendering|Material|SetCustomPrimitiveDataFloat (Variables|Character|GetMesh) 0 _time)
        (Development|PrintString (Utilities|String|ToString(Float) _time))))
    (else
      (Utilities|FlowControl|Sequence
        (:then_0
          (Timeline|Transition Reverse))
        (:then_1
          (Utilities|FlowControl|Delay 0.25)
          (CallFunction|UpdateMaterials (Variables|Default|GetDefaultMaterial)))))))

(event EventBeginPlay
  (|CallParentFunction)
  (Rendering|Material|SetCustomPrimitiveDataFloat (Variables|Character|GetMesh) 0 1.0)
  (Variables|Default|SetCooldownTime 14.0)
  (Networking|SwitchHasAuthority
    (:Authority
      (Variables|Default|SetDestructableActor "/Game/Blueprints/Pawns/BPD_Car.BPD_Car_C")
      (Variables|Default|SetHalf%20Size "170.000000,130.000000,70.000000"))))

(event Collision|EventActorBeginOverlap
  (params (OtherActor :type Actor%20Object%20Reference))
  (|CallParentFunction OtherActor) ; This node is disabled and will not be called.\nDrag off pins to build functionality.
)

(event EventTick
  (params (DeltaSeconds :type Float%20%28single-precision%29))
  (|CallParentFunction DeltaSeconds) ; This node is disabled and will not be called.\nDrag off pins to build functionality.
)

(event Input|ActionEvents|InputActionAbility
  (params (Key :type Key%20Structure :default "None"))
  (:Pressed
    (CallFunction|SRDecoy)))

(fn ConstructionScript
  (|CallParentFunction))

(fn UpdateMaterials
  (params (Material :type Material%20Interface%20Object%20Reference))
  (for _index (range 0 6)
    (Rendering|Material|SetMaterial (Variables|Character|GetMesh) _index Material)))