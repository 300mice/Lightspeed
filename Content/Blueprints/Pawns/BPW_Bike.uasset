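; Bike vehicle pawn that sets its vehicle type, cooldown and bike sound, plus server-only size, charge rates and destructible actor.
; Its ability input plays a sound, waits a second, then triggers a blink if the player is not dead.
; Outside cooldown, the blink zeroes velocity, teleports the bike forward without sweeping, and briefly pauses movement.
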(event Custom|BlinkAbility
  (if (not (Variables|Default|GetbCooldown))
    (CallFunction|StartCooldown)
    (Variables|Default|SetbMoving false)
    (|HandleTeleport_2)
    (Utilities|FlowControl|Delay 0.15)
    (Variables|Default|SetbMoving true)))

(event EventBeginPlay
  (Audio|Components|Audio|Play (Variables|Default|GetBike%20sound) 0.0)
  (|CallParentFunction)
  (Variables|Default|SetVehicleType 1)
  (Variables|Default|SetCooldownTime 16.0)
  (Networking|SwitchHasAuthority
    (:Authority
      (Variables|Default|SetHalf%20Size "180.000000,55.000000,50.000000")
      (Variables|Default|SetChargeIncreaseRate 0.5)
      (Variables|Default|SetChargeDecayRate 0.4)
      (Variables|Default|SetDestructableActor "/Game/Blueprints/Pawns/BPD_Bike.BPD_Bike_C"))))

(event Collision|EventActorBeginOverlap
  (params (OtherActor :type Actor%20Object%20Reference))
  (|CallParentFunction OtherActor) ; This node is disabled and will not be called.\nDrag off pins to build functionality.
)

(event EventTick
  (params (DeltaSeconds :type Float%20%28single-precision%29))
  (|CallParentFunction DeltaSeconds) ; This node is disabled and will not be called.\nDrag off pins to build functionality.
)

(event Input|ActionEvents|InputActionAbility
  (params (Key :type Key%20Structure :default "None"))
  (:Pressed
    (Audio|Components|Audio|Play (Variables|Default|Getability%20use) 0.0)
    (Utilities|FlowControl|Delay 1.0)
    (bind _asps_vehicle_player_state (Utilities|Casting|CastToPS_VehiclePlayerState (Variables|Default|GetPlayerState)))
    (if (not (Variables|/Game/Blueprints/_GameBP/PS_VehiclePlayerState.PS_VehiclePlayerState_C|GetbDead _asps_vehicle_player_state))
      (CallFunction|BlinkAbility)
      (Development|PrintString "Hello"))))

(fn ConstructionScript
  (|CallParentFunction))