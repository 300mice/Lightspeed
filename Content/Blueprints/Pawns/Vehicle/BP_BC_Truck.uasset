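; BP_BC_Truck is a playable truck vehicle pawn whose special ability drops a team-coloured wall.
; On BeginPlay it runs the parent setup, sets the ability cooldown, starts its audio and applies truck-specific turn and movement speeds.
; The Ability input calls SR_WallAbility, which, when off cooldown, starts the cooldown and spawns BP_WallAbility at SpawnPoint in the Team colour.
; MC_Spawn is an empty stub.
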(event Custom|SR_WallAbility
  (if (not (Variables|Default|GetbCooldown))
    (CallFunction|StartCooldown)
    (bind _returnvalue (Game|SpawnActorfromClass "/Game/Blueprints/Abilities/BP_WallAbility.BP_WallAbility_C" (Transformation|GetWorldTransform (Variables|Default|GetSpawnPoint)) "Undefined" 0 0))
    (Default|SetColour _returnvalue (Variables|Default|GetTeam))))

(event Custom|MC_Spawn)

(event Custom|SetUpTruck
  (Variables|Default|SetRotSpeed 0.4)
  (bind _output_get (Variables|Default|SetMoveSpeed 2.5e+03))
  (Variables|/Script/Engine.CharacterMovementComponent|SetMaxWalkSpeed (Variables|Character|GetCharacterMovement) _output_get))

(event EventBeginPlay
  (|CallParentFunction)
  (Variables|Default|SetCooldownTime 8.0)
  (Audio|Components|Audio|Play (Variables|Default|GetAudio) 0.0)
  (CallFunction|SetUpTruck))

(event Collision|EventActorBeginOverlap
  (params (OtherActor :type Actor%20Object%20Reference))
  (|CallParentFunction OtherActor) ; This node is disabled and will not be called.\nDrag off pins to build functionality.
)

(event EventTick
  (params (DeltaSeconds :type Float%20%28single-precision%29))
  (|CallParentFunction DeltaSeconds) ; This node is disabled and will not be called.\nDrag off pins to build functionality.
)

(event Input|ActionEvents|InputActionAbility
  (params (Key :type Key%20Structure :default "None"))
  (:Pressed
    (CallFunction|SRWallAbility)))

(fn ConstructionScript
  (|CallParentFunction))