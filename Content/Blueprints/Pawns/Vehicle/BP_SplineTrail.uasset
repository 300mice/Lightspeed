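; Trail actor that builds a spline mesh path from the positions of the vehicle it follows.
; Each WaypointHandle call appends a spline point at the vehicle's SpawnPoint, using its forward vector for tangents, and adds spline mesh segments between successive points after the first.
; GetDestroyed removes the actor.
; The construction-time mesh loop is disconnected, and the NodePositions RepNotify is empty.
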(event Custom|GetDestroyed
  (Actor|DestroyActor))

(event EventBeginPlay)

(event Collision|EventActorBeginOverlap
  (params (OtherActor :type Actor%20Object%20Reference)))

(fn ConstructionScript)

(fn WaypointHandle
  (bind _followvehicle (Variables|Default|GetFollowVehicle))
  (bind _spline (Variables|Default|GetSpline))
  (bind _spawnpoint (Variables|/Game/Blueprints/Pawns/Vehicle/BP_BaseCharacterClassTest.BP_BaseCharacterClassTest_C|GetSpawnPoint _followvehicle))
  (bind _returnvalue (Math|Vector|GetForwardVector _spawnpoint))
  (bind _result (Math|Integer|IncrementInt (Variables|Default|GetNextPoint))
    (:%20%20
      (Class|SplineComponent|AddPoint (Variables|Default|GetSpline) (Utilities|Struct|MakeSplinePoint (Math|Conversions|ToFloat(Integer) _result) (Transformation|GetWorldLocation _spawnpoint) _returnvalue _returnvalue "0.000000,0.000000,0.000000" "0.000000,0.000000,0.000000" "Curve") false)
      (if (not (== (Variables|Default|GetNextPoint) 1))
        (bind _returnvalue_2 (AddComponent|AddSplineMeshComponent true))
        (Utilities|FlowControl|Sequence
          (:then_0
            (if (> (Variables|Default|GetNextPoint) 1)
              (SplineMesh|SetStartandEnd _returnvalue_2 (.Location (Spline|GetLocationandTangentatSplinePoint _spline (- _result 1) "Local")) (.Tangent (Spline|GetLocationandTangentatSplinePoint _spline (- _result 1) "Local")) (.Location (Spline|GetLocationandTangentatSplinePoint _spline _result "Local")) (.Tangent (Spline|GetLocationandTangentatSplinePoint _spline _result "Local")) true :!class /Script/Engine.SplineMeshComponent))))))))

(fn OnRepNodePositions)