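; Bike vehicle pawn, a child Blueprint with a forward blink ability on a cooldown.
; On BeginPlay it starts its audio, and the authority sets its cooldown, rotation speed and movement speed.
; Ability input triggers the blink only while the player state is not dead.
; The blink zeroes velocity, jumps a fixed distance forward without sweeping for collision, and briefly pauses movement.
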(event Custom|BlinkAbility
  (if (not (Variables|Default|GetbCooldown))
    (CallFunction|StartCooldown)
    (Variables|Default|SetbMoving false)
    (|HandleTeleport)
    (Utilities|FlowControl|Delay 0.15)
    (Variables|Default|SetbMoving true)))

(event EventBeginPlay
  (|CallParentFunction)
  (Audio|Components|Audio|Play (Variables|Default|GetAudio) 0.0)
  (Networking|SwitchHasAuthority
    (:Authority
      (Variables|Default|SetCooldownTime 6.0)
      (Variables|Default|SetRotSpeed 0.3)
      (bind _output_get (Variables|Default|SetMoveSpeed 3.3e+03))
      (Variables|/Script/Engine.CharacterMovementComponent|SetMaxWalkSpeed (Variables|Character|GetCharacterMovement) _output_get))))

(event Collision|EventActorBeginOverlap
  (params (OtherActor :type Actor%20Object%20Reference))
  (|CallParentFunction OtherActor) ; This node is disabled and will not be called.\nDrag off pins to build functionality.
)

(event EventTick
  (params (DeltaSeconds :type Float%20%28single-precision%29))
  (|CallParentFunction DeltaSeconds) ; This node is disabled and will not be called.\nDrag off pins to build functionality.
)

(event Input|ActionEvents|InputActionAbility
  (params (Key :type Key%20Structure :default "None"))
  (:Pressed
    (bind _asps_vehicle_player_state (Utilities|Casting|CastToPS_VehiclePlayerState (Variables|Default|GetPlayerState)))
    (if (not (Variables|/Game/Blueprints/_GameBP/PS_VehiclePlayerState.PS_VehiclePlayerState_C|GetbDead _asps_vehicle_player_state))
      (CallFunction|BlinkAbility))))

(fn ConstructionScript
  (|CallParentFunction))