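; Base vehicle pawn, filed under OldVehicles, with Server/Client event pairs for start, steering and crashes.
; Horizontal axis input becomes yaw rotation, while forward input feeds AddMovementInput, oddly using actor location as direction.
; Hitting anything not tagged Floor destroys the vehicle and its spline trail reference and clears the controller's moving message.
; Trail spawning in HandleSpline is disconnected, and the cooldown timer has no caller here.
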(event OnComponentHit(Collider)
  (params (HitComponent :type Primitive%20Component%20Object%20Reference) (OtherActor :type Actor%20Object%20Reference) (OtherComp :type Primitive%20Component%20Object%20Reference) (NormalImpulse :type Vector :default "0, 0, 0") (Hit :type Hit%20Result%20Structure%20%28by%20ref%29))
  ;[1 1 1] Hit Detection
  (if (not (Actor|ActorHasTag OtherActor "Floor"))
    (CallFunction|ServerHitDetection)
    (Development|PrintString "HIT")))

(event OnComponentHit(Mesh)
  (params (HitComponent :type Primitive%20Component%20Object%20Reference) (OtherActor :type Actor%20Object%20Reference) (OtherComp :type Primitive%20Component%20Object%20Reference) (NormalImpulse :type Vector :default "0, 0, 0") (Hit :type Hit%20Result%20Structure%20%28by%20ref%29))
  ;[1 1 1] Hit Detection
  (if (not (Actor|ActorHasTag (stale OnComponentHit(Collider) OtherActor) "Floor"))
    (CallFunction|ServerHitDetection)
    (Development|PrintString "HIT")))

(event Custom|ServerHitDetection
  ;[1 1 1] Hit Detection
  (CallFunction|ClientHitDetection)
  (Actor|DestroyActor))

(event Custom|CooldownReset
  (Variables|Default|SetbCooldown false))

(event Custom|ClientStart
  (Class|BPIVehicleControls|SetMoving(Message) (Pawn|GetController) true))

(event Custom|StartCooldown
  (Variables|Default|SetbCooldown true)
  (Utilities|Time|SetTimerbyEvent (delegate Custom|CooldownReset) (Variables|Default|GetCooldownTime)))

(event Custom|ClientHitDetection
  ;[1 1 1] Hit Detection
  (Development|PrintString "Hello")
  (Actor|DestroyActor (Variables|Default|GetAs%20BP%20Spline%20Trail))
  (Class|BPIVehicleControls|SetMoving(Message) (Pawn|GetController) false))

(event Custom|ClientMoveForwards
  (params (NewParam :type Float%20%28single-precision%29)))

(event Custom|ServerMoveForwards
  (params (NewParam :type Float%20%28single-precision%29))
  (Pawn|Input|AddMovementInput (Transformation|GetActorLocation) NewParam true))

(event Custom|RecieveMouseInput
  (params (movementRot :type Float%20%28single-precision%29))
  (CallFunction|ServerRotateMovement (stale Input|AxisEvents|InputAxismoveHorizontal AxisValue)))

(event Custom|ServerRotateMovement
  (params (NewParam :type Float%20%28single-precision%29))
  (CallFunction|ClientRotateMovement NewParam))

(event Custom|ClientRotateMovement
  (params (NewParam :type Float%20%28single-precision%29))
  (CallFunction|MouseSteeringControls NewParam))

(event Custom|ServerStart
  (CallFunction|ClientStart))

(event EventBeginPlay
  (Networking|SwitchHasAuthority
    (:Authority
      (CallFunction|ClientStart))
    (:Remote
      (CallFunction|ServerStart))))

(event EventTick
  (params (DeltaSeconds :type Float%20%28single-precision%29)))

(event Input|AxisEvents|InputAxismoveHorizontal
  (params (AxisValue :type Float%20%28single-precision%29))
  (Networking|SwitchHasAuthority
    (:Authority
      (CallFunction|ClientRotateMovement AxisValue)
      (CallFunction|ServerRotateMovement AxisValue))
    (:Remote
      (CallFunction|ServerRotateMovement AxisValue))))

(event Input|AxisEvents|InputAxisMoveForward
  (params (AxisValue :type Float%20%28single-precision%29))
  (CallFunction|ServerMoveForwards AxisValue))

(fn ConstructionScript)

(fn HandleSpline
  (Utilities|Time|ClearandInvalidateTimerbyHandle (Variables|Default|GetSplineTimer))
  (bind _returnvalue (Game|SpawnActorfromClass "/Game/Blueprints/Pawns/Vehicle/BP_SplineTrail.BP_SplineTrail_C" (Transformation|GetWorldTransform (Variables|Default|GetSpawnPoint)) "AlwaysSpawn" 0 0))
  (Variables|Default|SetAs%20BP%20Spline%20Trail _returnvalue))

(fn MouseSteeringControls
  (params (Delta%20Rotation%20Z%20%28Yaw%29 :type Float%20%28single-precision%29))
  ;[1 1 1] Get Viewport size and divide mouse position by half so that center = 0, left = -0.5, right = 0.5
  (Class|Actor|AddActorWorldRotation (Math|Rotator|MakeRotator 0.0 0.0 Delta%20Rotation%20Z%20%28Yaw%29)))

(fn MoveForward
  (Transformation|SetActorLocation (+ (Transformation|GetActorForwardVector) (Transformation|GetActorLocation)) false false))