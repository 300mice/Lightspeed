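; Test base vehicle character for a networked car game that drives forward constantly once the game state's round is playing, steering by horizontal mouse position.
; The server sets movement, and non-floor capsule hits increment the dead count, mark the car dead and destroy its spline trail.
; RepNotifies spawn a BP_SplineTrail when movement starts, clear the trail timer when it stops, and destroy the actor on death.
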(event OnComponentHit(CapsuleComponent)
  (params (HitComponent :type Primitive%20Component%20Object%20Reference) (OtherActor :type Actor%20Object%20Reference) (OtherComp :type Primitive%20Component%20Object%20Reference) (NormalImpulse :type Vector :default "0, 0, 0") (Hit :type Hit%20Result%20Structure%20%28by%20ref%29))
  (Networking|SwitchHasAuthority
    (:Authority
      (if (not (Actor|ActorHasTag OtherActor "Floor"))
        (bind _asgs_car_game (Utilities|Casting|CastToGS_CarGame (Game|GetGameState)))
        (Variables|/Game/Blueprints/_GameBP/GS_CarGame.GS_CarGame_C|SetPlayersDead _asgs_car_game (+ (Variables|/Game/Blueprints/_GameBP/GS_CarGame.GS_CarGame_C|GetPlayersDead _asgs_car_game) 1))
        (Variables|Default|SetbDead true)
        (Variables|Default|SetbMoving false)
        (Default|GetDestroyed (Variables|Default|GetAs%20BP%20Spline%20Trail))))))

(event Custom|Mouse)

(event Custom|CooldownReset
  (Variables|Default|SetbCooldown false))

(event Custom|StartCooldown
  (Variables|Default|SetbCooldown true)
  (Utilities|Time|SetTimerbyEvent (delegate Custom|CooldownReset) (Variables|Default|GetCooldownTime)))

(event Custom|GameStarted)

(event EventBeginPlay
  (Networking|SwitchHasAuthority))

(event Collision|EventActorBeginOverlap
  (params (OtherActor :type Actor%20Object%20Reference)))

(event EventTick
  (params (DeltaSeconds :type Float%20%28single-precision%29))
  (if (Variables|Default|GetbMoving)
    ;[1 1 1] Car movement on tick
    (Pawn|Input|AddMovementInput (Transformation|GetActorForwardVector) 1.0 true)
    (bind _returnvalue (CallFunction|FindRotation))
    (Pawn|Input|AddControllerYawInput _returnvalue)
    (else
      ;[1 1 1] Starts moving when the game state says its ok
      (Networking|SwitchHasAuthority
        (:Authority
          (bind _asgs_car_game (Utilities|Casting|CastToGS_CarGame (Game|GetGameState)))
          (Variables|Default|SetbMoving (Variables|/Game/Blueprints/_GameBP/GS_CarGame.GS_CarGame_C|GetRoundPlaying _asgs_car_game)))))))

(fn ConstructionScript)

(fn HandleSpline)

(fn FindRotation
  (bind _returnvalue (Class|WidgetLayoutLibrary|GetMousePositiononViewport))
  (bind _output_get (Variables|Default|SetMovementFloat (- (/ (* (.x _returnvalue) (Class|WidgetLayoutLibrary|GetViewportScale)) (.x (Viewport|GetViewportSize))) 0.5)))
  (return (/ _output_get 5.0)))

(fn OnRepSplineTimer)

(fn OnRepasBPSplineTrail)

(fn OnRepBMoving
  (if (Variables|Default|GetbMoving)
    (Game|SpawnActorfromClass "/Game/Blueprints/Pawns/Vehicle/BP_SplineTrail.BP_SplineTrail_C" (Transformation|GetWorldTransform (Variables|Default|GetSpawnPoint)) "AlwaysSpawn" 0 0)
    (else
      (Utilities|Time|ClearandInvalidateTimerbyHandle (Variables|Default|GetSplineTimer)))))

(fn OnRepBDead
  (if (Variables|Default|GetbDead)
    (Actor|DestroyActor)))