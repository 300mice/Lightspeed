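; Field System actor that fires an explosion on BeginPlay to break and launch Chaos destructible geometry.
; It plays an explosion cue at the world origin, then applies external cluster strain within the Sphere component's radius.
; A radial velocity field scaled by ExplosionForce, culled outside that sphere, pushes pieces from a point behind its center, biasing debris forward.
; The Explode event is an empty stub.
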(event Custom|Explode)

(event EventBeginPlay
  (bind _fieldsystemcomponent (Variables|Field|GetFieldSystemComponent))
  (bind _radialfalloff (Variables|Default|GetRadialFalloff))
  (bind _sphere (Variables|Default|GetSphere))
  (bind _sphere_2 (Variables|Default|GetSphere))
  (bind _returnvalue (Components|Sphere|GetScaledSphereRadius _sphere))
  (bind _returnvalue_2 (Transformation|GetWorldLocation _sphere))
  (bind _returnvalue_3 (Field|SetRadialFalloff _radialfalloff 5e+07 0.0 1.0 0.0 _returnvalue _returnvalue_2 "Field_FallOff_None"))
  (Audio|PlaySoundatLocation "/Game/StarterContent/Audio/Explosion_Cue.Explosion_Cue" "0, 0, 0" "0, 0, 0" 1.0 1.0 0.0 0 0 0 0)
  (Class|FieldSystemComponent|ApplyPhysicsField _fieldsystemcomponent true "Field_ExternalClusterStrain" 0 _returnvalue_3)
  (Class|FieldSystemComponent|ApplyPhysicsField _fieldsystemcomponent true "Field_LinearVelocity" 0 (Field|SetCullingField (Variables|Default|GetCullingField) _returnvalue_3 (Field|SetRadialVector (Variables|Default|GetRadialVector) (Variables|Default|GetExplosionForce) (+ (* (Math|Vector|GetForwardVector _sphere_2) -2e+02) (Transformation|GetWorldLocation _sphere_2))) "Field_Culling_Outside")))

(event Collision|EventActorBeginOverlap
  (params (OtherActor :type Actor%20Object%20Reference)))

(event EventTick
  (params (DeltaSeconds :type Float%20%28single-precision%29)))

(fn ConstructionScript)