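; Base character for a multiplayer trail-leaving vehicle that constantly drives forward while moving and ends the round on hitting anything not tagged Floor.
; Tick applies movement and steering; Boost and Break share a Charge meter, trading speed against turn rate while camera FOV shifts.
; A looping server timer updates Position, whose RepNotify adds cubes to a shared BP_InstancedTrail.
; Team RepNotify sets the material; server-stored start transform supports restarts.
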(event OnComponentHit(CapsuleComponent)
  (params (HitComponent :type Primitive%20Component%20Object%20Reference) (OtherActor :type Actor%20Object%20Reference) (OtherComp :type Primitive%20Component%20Object%20Reference) (NormalImpulse :type Vector :default "0, 0, 0") (Hit :type Hit%20Result%20Structure%20%28by%20ref%29))
  ;[1 1 1] We need to register the hit on the server and delete the actor
  (if (Utilities|IsValid OtherActor)
    (Networking|SwitchHasAuthority
      (:Authority
        (if (not (Actor|ActorHasTag OtherActor "Floor"))
          (Class|BPIRoundDependent|EndRound(Message) (Variables|GetPlayerState)))))))

(event Custom|SR_SetTeam
  (params (Team :type Integer))
  ;[1 0.1032 0.143] Team & Colour
  (Variables|Default|SetTeam Team))

(event Custom|CooldownReset
  ;[0.2904 1 0.9602] Ability Cooldowns
  (Variables|Default|SetbCooldown false))

(event Custom|StartCooldown
  ;[0.2904 1 0.9602] Ability Cooldowns
  (Variables|Default|SetbCooldown true)
  (Utilities|Time|SetTimerbyEvent (delegate Custom|CooldownReset) (Variables|Default|GetCooldownTime)))

(event Custom|SR_AddSteeringPower
  (params (Amount :type Float%20%28single-precision%29))
  (bind _rotspeed (Variables|Default|GetRotSpeed))
  ;[0.2595 1 0.1295] Movement
  (Variables|Default|SetSteeringPower (Math|Float|Clamp(Float) (+ (/ (Math|Float|Clamp(Float) Amount -1.0) 3e+01) (Variables|Default|GetSteeringPower)) (* -1 _rotspeed) _rotspeed)))

(event Custom|SpawnTrail
  ;[0.7353 0.1502 1] If server - set timer, everyone else finds the Trail Object in the map :D
  (if (Variables|Default|GetbMoving)
    (Variables|Default|SetPosition (Transformation|GetWorldTransform (Variables|Default|GetSpawnPoint)))))

(event Custom|SR_Moving
  (params (Moving :type Boolean))
  ;[1 0.7259 0.1289] Moving
  (Variables|Default|SetbMoving Moving))

(event Custom|SR_Break
  (params (Pressed :type Boolean))
  (bind _charactermovement (Variables|Character|GetCharacterMovement))
  (bind _charactermovement_2 (Variables|Character|GetCharacterMovement))
  (if Pressed
    (if (and (> (Variables|Default|GetCharge) 2e+01) (not (Variables|Default|GetBoost)))
      (Variables|/Script/Engine.CharacterMovementComponent|SetMaxWalkSpeed _charactermovement (/ (Variables|/Script/Engine.CharacterMovementComponent|GetMaxWalkSpeed _charactermovement) 1.5))
      (Variables|Default|SetBreak true)
      (Variables|Default|SetRotSpeed (* (Variables|Default|GetRotSpeed) 1.5)))
    (else
      (Variables|/Script/Engine.CharacterMovementComponent|SetMaxWalkSpeed _charactermovement_2 (* (Variables|/Script/Engine.CharacterMovementComponent|GetMaxWalkSpeed _charactermovement_2) 1.5))
      (Variables|Default|SetBreak false)
      (Variables|Default|SetRotSpeed (/ (Variables|Default|GetRotSpeed) 1.5)))))

(event Custom|SR_Boost
  (params (Pressed :type Boolean))
  (bind _charactermovement (Variables|Character|GetCharacterMovement))
  (bind _charactermovement_2 (Variables|Character|GetCharacterMovement))
  (if Pressed
    (if (and (> (Variables|Default|GetCharge) 2e+01) (not (Variables|Default|GetBreak)))
      (Variables|/Script/Engine.CharacterMovementComponent|SetMaxWalkSpeed _charactermovement (* (Variables|/Script/Engine.CharacterMovementComponent|GetMaxWalkSpeed _charactermovement) 1.5))
      (Variables|Default|SetBoost true)
      (Variables|Default|SetRotSpeed (/ (Variables|Default|GetRotSpeed) 1.5)))
    (else
      (Variables|/Script/Engine.CharacterMovementComponent|SetMaxWalkSpeed _charactermovement_2 (/ (Variables|/Script/Engine.CharacterMovementComponent|GetMaxWalkSpeed _charactermovement_2) 1.5))
      (Variables|Default|SetBoost false)
      (Variables|Default|SetRotSpeed (* (Variables|Default|GetRotSpeed) 1.5)))))

(event Custom|SR_DepleteCharge
  (Variables|Default|SetCharge (Math|Float|Clamp(Float) (- (Variables|Default|GetCharge) 0.5) 0.0 1e+02)))

(event Custom|SR_IncreaseCharge
  (Variables|Default|SetCharge (Math|Float|Clamp(Float) (+ (Variables|Default|GetCharge) 0.1) 0.0 1e+02)))

(event EventBeginPlay
  ;[0.7353 0.1502 1] If server - set timer, everyone else finds the Trail Object in the map :D
  (Networking|SwitchHasAuthority
    (:Authority
      (Utilities|Time|SetTimerbyEvent (delegate Custom|SpawnTrail) 0.01 true))
    (:Remote
      _))
  (bind _returnvalue (Actor|GetActorOfClass "/Game/Blueprints/Abilities/BP_InstancedTrail.BP_InstancedTrail_C"))
  (Variables|Default|SetTrail _returnvalue)
  (Networking|SwitchHasAuthority
    (:Authority
      (Variables|Default|SetstartPos (Transformation|GetActorTransform)))))

(event EventTick
  (params (DeltaSeconds :type Float%20%28single-precision%29))
  (bind _camera1 (Variables|Default|GetCamera1))
  (bind _camera1_2 (Variables|Default|GetCamera1))
  (bind _camera1_3 (Variables|Default|GetCamera1))
  ;[0.2595 1 0.1295] Movement
  ;;[1 1 1] Car movement on tick
  (if (Variables|Default|GetbMoving)
    (Pawn|Input|AddMovementInput (Transformation|GetActorForwardVector) 1.0 true)
    (Pawn|Input|AddControllerYawInput (Variables|Default|GetSteeringPower))
    (if (or (Variables|Default|GetBreak) (Variables|Default|GetBoost))
      (CallFunction|SRDepleteCharge)
      (else
        (CallFunction|SRIncreaseCharge)))
    (if (== (Variables|Default|GetCharge) 0.0)
      (CallFunction|SRBreak false)
      (CallFunction|SRBoost false))
    (if (Variables|Default|GetBoost)
      (Camera|SetFieldOfView _camera1 (Math|Interpolation|FInterpTo (Variables|/Script/Engine.CameraComponent|GetFieldOfView _camera1) 1.1e+02 (Utilities|Time|GetWorldDeltaSeconds) 5.0))
      (elif (Variables|Default|GetBreak)
        (Camera|SetFieldOfView _camera1_2 (Math|Interpolation|FInterpTo (Variables|/Script/Engine.CameraComponent|GetFieldOfView _camera1_2) 8e+01 (Utilities|Time|GetWorldDeltaSeconds) 5.0))
        (else
          (Camera|SetFieldOfView _camera1_3 (Math|Interpolation|FInterpTo (Variables|/Script/Engine.CameraComponent|GetFieldOfView _camera1_3) 9e+01 (Utilities|Time|GetWorldDeltaSeconds) 3.0)))))))

(event EventSetMoving
  (params (Moving :type Boolean))
  ;[1 0.7259 0.1289] Moving
  (CallFunction|SRMoving Moving))

(event EventDestroyTrail
  (Default|DestroyTrail (Variables|Default|GetTrail) (Variables|Default|GetTeam))
  (CallFunction|SRMoving false))

(event EventSetColour
  (params (Team :type Integer))
  ;[1 0.1032 0.143] Team & Colour
  (CallFunction|SRSetTeam Team))

(event EventRestartVehicle
  (Transformation|SetActorTransform (Variables|Default|GetstartPos)))

(event Input|ActionEvents|InputActionBreak
  (params (Key :type Key%20Structure :default "None"))
  (:Pressed
    (CallFunction|SRBreak true))
  (:Released
    (CallFunction|SRBreak false)))

(event Input|ActionEvents|InputActionBoost
  (params (Key :type Key%20Structure :default "None"))
  (:Pressed
    (CallFunction|SRBoost true))
  (:Released
    (CallFunction|SRBoost false)))

(event Input|AxisEvents|InputAxisTurnRight
  (params (AxisValue :type Float%20%28single-precision%29))
  ;[0.2595 1 0.1295] Movement
  (if (!= (Class|Actor|GetInputAxisKeyValue) 0.0)
    (Pawn|Input|AddControllerYawInput (* AxisValue (Variables|Default|GetRotSpeed)))
    (Variables|Default|SetSteeringPower 0.0)
    (else
      (CallFunction|SRAddSteeringPower AxisValue))))

(fn ConstructionScript)

(fn HandleSpline)

(fn FindRotation
  (bind _returnvalue (Class|WidgetLayoutLibrary|GetMousePositiononViewport))
  (bind _output_get (Variables|Default|SetMovementFloat (- (/ (* (.x _returnvalue) (Class|WidgetLayoutLibrary|GetViewportScale)) (.x (Viewport|GetViewportSize))) 0.5)))
  (return (/ _output_get 5.0)))

(fn OnRepSplineTimer)

(fn OnRepasBPSplineTrail)

(fn OnRepBMoving)

(fn OnRepBDead
  (if (Variables|Default|GetbDead)
    (Default|DestroyTrail (Variables|Default|GetTrail) (Variables|Default|GetTeam))))

(fn OnRepTrail)

(fn OnRepPosition
  (if (Utilities|IsValid (Variables|Default|GetTrail))
    (Default|SpawnCube (Variables|Default|GetTrail) (Variables|Default|GetPosition) (Variables|Default|GetTeam))))

(fn OnRepTeam
  (Rendering|Material|SetMaterial (Variables|Default|GetStaticMesh) 0 (Utilities|Array|Get(acopy) (Variables|Default|GetColourMaterials) (Variables|Default|GetTeam))))