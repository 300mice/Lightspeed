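; Base vehicle pawn for a multiplayer trail-leaving driving game, with automatic throttle, boost and brake.
; While moving, the server samples the trail point on a looping timer, and Position's OnRep adds a team cube to the shared BP_InstancedTrail.
; Tick box-traces for obstacles, ending the round through PlayerState on a hit.
; Otherwise it applies throttle or handbrake, adjusts Charge and interpolates camera FOV by movement mode.
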(event Custom|SR_SetTeam
  (params (Team :type Integer))
  ;[1 0.07011 0.22] Team & Colour
  (Variables|Default|SetTeam Team))

(event Custom|CooldownReset
  ;[0.2904 1 0.9602] Ability Cooldowns
  (Variables|Default|SetbCooldown false))

(event Custom|DestroyVehicle
  ;[0.7352 1 0.5501] Detect Hit on Server, then end round on Player State
  (Class|BPIRoundDependent|EndRound(Message) (Variables|GetPlayerState)))

(event Custom|StartCooldown
  ;[0.2904 1 0.9602] Ability Cooldowns
  (Variables|Default|SetbCooldown true)
  (Utilities|Time|SetTimerbyEvent (delegate Custom|CooldownReset) (Variables|Default|GetCooldownTime)))

(event Custom|SR_AddSteeringPower
  (params (Amount :type Float%20%28double-precision%29))
  ;[0.4362 0.1726 1] Steering
  (bind _output_get (Variables|Default|SetSteeringPower (Math|Float|Clamp(Float) (+ (/ (Math|Float|Clamp(Float) Amount -1.0) 25.0) (Variables|Default|GetSteeringPower)) -1.0)))
  (Class|ChaosVehicleMovementComponent|SetSteeringInput (Variables|Default|GetVehicleMovementComponent) _output_get))

(event Custom|SpawnTrail
  ;[0.7353 0.1502 1] If server - set timer, everyone else finds the Trail Object in the map :D
  (if (Variables|Default|GetbMoving)
    (Variables|Default|SetPosition (Transformation|GetWorldTransform (Variables|Default|GetTrailPoint)))))

(event Custom|SR_Moving
  (params (Moving :type Boolean))
  ;[1 0.7222 0.1142] Moving
  (Variables|Default|SetbMoving Moving))

(event Custom|OnTakeAnyDamage_Event
  (params (DamagedActor :type Actor%20Object%20Reference) (Damage :type Float%20%28single-precision%29) (DamageType :type Damage%20Type%20Object%20Reference) (InstigatedBy :type Controller%20Object%20Reference) (DamageCauser :type Actor%20Object%20Reference))
  (Development|PrintString "Hello" true true "(R=1.000000,G=0.000000,B=0.138428,A=1.000000)"))

(event Custom|SR_DepleteCharge
  ;[1 0.1941 0.5553] Adjust Boost & Brake Charge amount based on usage
  (Variables|Default|SetCharge (Math|Float|Clamp(Float) (- (Variables|Default|GetCharge) 0.5) 0.0 1e+02)))

(event Custom|SR_IncreaseCharge
  ;[1 0.1941 0.5553] Adjust Boost & Brake Charge amount based on usage
  (Variables|Default|SetCharge (Math|Float|Clamp(Float) (+ (Variables|Default|GetCharge) 0.1) 0.0 1e+02)))

(event EventBeginPlay
  ;[0.7353 0.1502 1] If server - set timer, everyone else finds the Trail Object in the map :D
  (Networking|SwitchHasAuthority
    (:Authority
      (Utilities|Time|SetTimerbyEvent (delegate Custom|SpawnTrail) 0.01 true))
    (:Remote
      _))
  (bind _returnvalue (Actor|GetActorOfClass "/Game/Blueprints/Abilities/BP_InstancedTrail.BP_InstancedTrail_C"))
  (Variables|Default|SetTrail _returnvalue)
  (Networking|SwitchHasAuthority
    (:Authority
      (Variables|Default|SetstartPos (Transformation|GetActorTransform))
      (EventDispatchers|BindEventtoOnTakeAnyDamage (delegate Custom|OnTakeAnyDamage_Event)))))

(event Collision|EventActorBeginOverlap
  (params (OtherActor :type Actor%20Object%20Reference)))

(event EventTick
  (params (DeltaSeconds :type Float%20%28single-precision%29))
  (bind _mesh (Variables|Character|GetMesh))
  (bind _returnvalue (Transformation|GetWorldLocation _mesh))
  (if (Variables|Default|GetbMoving)
    (bind (_outhit _returnvalue_2) (Collision|BoxTraceByChannel (+ _returnvalue "10.000000,0.000000,150.000000") (+ _returnvalue "10.000000,0.000000,150.000000") (Variables|Default|GetHalf%20Size) (Transformation|GetWorldRotation (Variables|Character|GetMesh)) "TraceTypeQuery1" false (Utilities|Array|MakeArray self) "ForOneFrame"))
    (if (Utilities|IsValid (.HitActor (Collision|BreakHitResult _outhit)))
      (if (and _returnvalue_2 (or (not (Actor|ActorHasTag (.HitActor (Collision|BreakHitResult _outhit)) "Floor")) (> (.y (.ImpactNormal (Collision|BreakHitResult _outhit))) 1.0)))
        (CallFunction|DestroyVehicle)
        (Development|PrintString "Hello" true true "(R=1.000000,G=0.304238,B=0.164261,A=1.000000)" 2e+02)
        (else
          (if (!= (Variables|Default|GetMovementMode) 0) :!label _label
            (CallFunction|SRDepleteCharge)
            (else
              (CallFunction|SRIncreaseCharge)))
          (Utilities|FlowControl|Sequence
            (:then_0
              (if (Variables|Default|Getbrake)
                (Class|ChaosVehicleMovementComponent|SetHandbrakeInput (Variables|Default|GetVehicleMovementComponent) true)
                (Class|ChaosVehicleMovementComponent|SetThrottleInput (Variables|Default|GetVehicleMovementComponent) 0.0)
                (else
                  (Class|ChaosVehicleMovementComponent|SetHandbrakeInput (Variables|Default|GetVehicleMovementComponent) false)
                  (Class|ChaosVehicleMovementComponent|SetThrottleInput (Variables|Default|GetVehicleMovementComponent) 0.5))))
            (:then_1
              (if (Variables|Default|Getboost)
                (Class|ChaosVehicleMovementComponent|IncreaseThrottleInput (Variables|Default|GetVehicleMovementComponent) 1.0)))
            (:then_2
              (switch int (Variables|Default|GetMovementMode)
                (:Default
                  (CallFunction|InterptoFOV 9e+01 :!label _label_2))
                (:0
                  (goto _label_2))
                (:1
                  (CallFunction|InterptoFOV 1.1e+02))
                (:2
                  (CallFunction|InterptoFOV 8e+01)))))))
      (else
        (goto _label)))
    (else
      (Variables|/Script/Engine.MovementComponent|SetVelocity (Variables|Default|GetVehicleMovementComponent) "0, 0, 0")
      (Class|ChaosVehicleMovementComponent|SetThrottleInput (Variables|Default|GetVehicleMovementComponent) 0.0))))

(event EventSetColour
  (params (Team :type Integer))
  ;[1 0.07011 0.22] Team & Colour
  (CallFunction|SRSetTeam Team))

(event EventSetMoving
  (params (Moving :type Boolean))
  ;[1 0.7222 0.1142] Moving
  (Variables|Default|SetbMoving Moving)
  (CallFunction|SRMoving Moving))

(event EventRestartVehicle
  ;[1 0.739 0.2663] Restart Vehicle to Starting Position
  (Transformation|SetActorTransform (Variables|Default|GetstartPos) false true))

(event Input|ActionEvents|InputActionBreak
  (params (Key :type Key%20Structure :default "None"))
  (:Pressed
    (Variables|Default|Setbrake true)
    (Variables|Default|SetMovementMode 2))
  (:Released
    (Variables|Default|Setbrake false)
    (Variables|Default|SetMovementMode 0)))

(event Input|ActionEvents|InputActionBoost
  (params (Key :type Key%20Structure :default "None"))
  (:Pressed
    (Variables|Default|Setboost true)
    (Variables|Default|SetMovementMode 1))
  (:Released
    (Variables|Default|Setboost false)
    (Variables|Default|SetMovementMode 0)))

(event Input|AxisEvents|InputAxisTurnRight
  (params (AxisValue :type Float%20%28single-precision%29))
  ;[0.4362 0.1726 1] Steering
  (if (!= (Class|Actor|GetInputAxisKeyValue) 0.0)
    (Class|ChaosVehicleMovementComponent|SetSteeringInput (Variables|Default|GetVehicleMovementComponent) AxisValue)
    (Variables|Default|SetSteeringPower 0.0)
    (else
      (CallFunction|SRAddSteeringPower AxisValue))))

(fn ConstructionScript)

(fn OnRepPosition
  (if (Utilities|IsValid (Variables|Default|GetTrail))
    (Default|SpawnCube (Variables|Default|GetTrail) (Variables|Default|GetPosition) (Variables|Default|GetTeam))))

(fn InterptoFOV
  (params (TargetFOV :type Float%20%28double-precision%29))
  (bind _camera (Variables|Default|GetCamera))
  (Camera|SetFieldOfView _camera (Math|Interpolation|FInterpTo (Variables|/Script/Engine.CameraComponent|GetFieldOfView _camera) TargetFOV (Utilities|Time|GetWorldDeltaSeconds) 5.0)))