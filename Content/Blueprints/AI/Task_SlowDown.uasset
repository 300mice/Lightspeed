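; Behavior tree task that makes an AI-driven wheeled vehicle brake when something blocks the path ahead.
; It caches the vehicle, then sphere-traces forward from its ForwardDetection component, ignoring itself and actors from the game mode's GetFloorMessage.
; A hit sets the brake and a miss releases it.
; The task finishes successfully right away, with a brake release scheduled after a short delay.
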(event EventReceiveExecuteAI
  (params (OwnerController :type AI%20Controller%20Object%20Reference) (ControlledPawn :type Pawn%20Object%20Reference))
  (if (Utilities|IsValid (Variables|Default|GetVehicle))
    _
    (else
      (bind _asbp_wheeled_vehicle_base (Utilities|Casting|CastToBP_WheeledVehicleBase ControlledPawn))
      (Variables|Default|SetVehicle _asbp_wheeled_vehicle_base)))
  (bind _returnvalue (CallFunction|CollisionLineTrace))
  (if _returnvalue
    (Default|SRBrake (Variables|Default|GetVehicle) true)
    (else
      (Default|SRBrake (Variables|Default|GetVehicle) false)))
  (AI|BehaviorTree|FinishExecute true)
  (Utilities|FlowControl|Delay 0.7)
  (Default|SRBrake (Variables|Default|GetVehicle) false))

(fn CollisionLineTrace
  (bind _vehicle (Variables|Default|GetVehicle))
  (bind _forwarddetection (Variables|/Game/Blueprints/Pawns/BP_WheeledVehicleBase.BP_WheeledVehicleBase_C|GetForwardDetection _vehicle))
  (bind _returnvalue (Transformation|GetWorldLocation _forwarddetection))
  (bind _floor (Class|BPIGameMode|GetFloor(Message) (Game|GetGameMode)))
  (LocalVariables|SetNewLocalVar_0 _floor)
  (Utilities|Array|Add (LocalVariables|GetNewLocalVar_0) (Variables|Default|GetVehicle))
  (bind _returnvalue_2 (Collision|SphereTraceByChannel _returnvalue (+ _returnvalue (* (Math|Vector|GetForwardVector _forwarddetection) 4.5e+03)) 1e+02 "TraceTypeQuery1" false (LocalVariables|GetNewLocalVar_0) "ForOneFrame"))
  (return _returnvalue_2))