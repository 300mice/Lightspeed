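; An EQS context that supplies a set of hit locations around the querier for AI environment queries.
; It fires six evenly spaced, very long Visibility line traces in yaw around the actor's forward vector and stores each hit location.
; A miss stores the negated, scaled forward vector, without adding the actor's location.
; Traces draw for one frame and the first result is printed for debugging.
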(fn ProvideLocationsSet
  (params (QuerierObject :type Object%20Object%20Reference) (QuerierActor :type Actor%20Object%20Reference))
  (bind _returnvalue (Transformation|GetActorForwardVector QuerierActor))
  (bind _returnvalue_2 (Transformation|GetActorLocation QuerierActor))
  (bind _resulting_location_set (Variables|Default|GetResulting%20Location%20Set))
  (bind _resulting_location_set_2 (Variables|Default|GetResulting%20Location%20Set))
  (Utilities|Array|Clear (Variables|Default|GetResulting%20Location%20Set))
  (for _index (range 0 5)
    (bind (_outhit _returnvalue_3) (Collision|LineTraceByChannel _returnvalue_2 (+ _returnvalue_2 (* (Math|Vector|RotateVector _returnvalue (Math|Rotator|MakeRotator 0.0 0.0 (Math|Conversions|ToFloat(Integer) (* _index (/ 360 6))))) 1e+06)) "TraceTypeQuery1" false 0 "ForOneFrame"))
    (if _returnvalue_3
      (Utilities|Array|Add _resulting_location_set_2 (.location _outhit))
      (else
        (Utilities|Array|Add _resulting_location_set_2 (* _returnvalue -5e+03)))))
  (Development|PrintString (Utilities|String|ToString(Vector) (Utilities|Array|Get(acopy) _resulting_location_set)))
  (return _resulting_location_set))