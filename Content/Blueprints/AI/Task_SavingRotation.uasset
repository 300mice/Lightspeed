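; Behavior tree task that yaws an AI vehicle away from obstacles ahead, one rotation step per execution.
; Sphere traces from its left and right detection components, ignoring the game mode's floor actors, fail the task when neither hits.
; Otherwise, long side line traces compare impact distances, and the vehicle turns toward the farther one by Speed times delta time.
; GetLargerDistance is a stub returning false; both adjust functions are identical, so LeftAngle alone sets direction.
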(event EventReceiveExecuteAI
  (params (OwnerController :type AI%20Controller%20Object%20Reference) (ControlledPawn :type Pawn%20Object%20Reference))
  (bind _output_get (Variables|Default|SetControlled%20Pawn ControlledPawn))
  (bind _asbp_base_character_class_test (Utilities|Casting|CastToBP_BaseCharacterClass _output_get))
  (Variables|Default|SetAs%20BP%20Base%20Vehicle _asbp_base_character_class_test)
  (|CeckForCornerCollisions_2)
  (|GetBiggerSide_2)
  (bind _rightislarger (CallFunction|GetLargerDistance))
  (if _rightislarger
    (CallFunction|AdjustTurnAngleLeft 0.0)
    (else
      (CallFunction|AdjustTurnAngleRight 0.0)))
  (AI|BehaviorTree|FinishExecute true))

(fn GetLargerDistance
  (return false))

(fn AdjustTurnAngleRight
  (params (ChosenAngle :type Float%20%28single-precision%29))
  (if (Variables|Default|GetbLeftAngle)
    (Class|Actor|AddActorWorldRotation (Variables|Default|GetAs%20BP%20Base%20Vehicle) (Math|Rotator|MakeRotator 0.0 0.0 (* -1 (* (Variables|Default|GetSpeed) (Utilities|Time|GetWorldDeltaSeconds)))))
    (else
      (Class|Actor|AddActorWorldRotation (Variables|Default|GetAs%20BP%20Base%20Vehicle) (Math|Rotator|MakeRotator 0.0 0.0 (* (Variables|Default|GetSpeed) (Utilities|Time|GetWorldDeltaSeconds)))))))

(fn AdjustTurnAngleLeft
  (params (ChosenAngle :type Float%20%28single-precision%29))
  (if (Variables|Default|GetbLeftAngle)
    (Class|Actor|AddActorWorldRotation (Variables|Default|GetAs%20BP%20Base%20Vehicle) (Math|Rotator|MakeRotator 0.0 0.0 (* -1 (* (Variables|Default|GetSpeed) (Utilities|Time|GetWorldDeltaSeconds)))))
    (else
      (Class|Actor|AddActorWorldRotation (Variables|Default|GetAs%20BP%20Base%20Vehicle) (Math|Rotator|MakeRotator 0.0 0.0 (* (Variables|Default|GetSpeed) (Utilities|Time|GetWorldDeltaSeconds)))))))

(fn CollisionLineTrace
  (params (Target :type Scene%20Component%20Object%20Reference) (Distance :type Float%20%28single-precision%29))
  (bind _returnvalue (Transformation|GetWorldLocation Target))
  (bind _floor (Class|BPIGameMode|GetFloor(Message) (Game|GetGameMode)))
  (LocalVariables|SetNewLocalVar_0 _floor)
  (Utilities|Array|Add (LocalVariables|GetNewLocalVar_0) (Variables|Default|GetControlled%20Pawn))
  (bind (_outhit _returnvalue_2) (Collision|SphereTraceByChannel _returnvalue (+ (* (Math|Vector|GetForwardVector Target) Distance) _returnvalue) 1e+02 "TraceTypeQuery1" false (LocalVariables|GetNewLocalVar_0) "ForOneFrame"))
  (return _outhit _returnvalue_2))