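; Behavior tree task that makes an AI-controlled BP_WheeledVehicleBase cast its ability when something is in front of it.
; Caches the vehicle, then box-traces a short distance from its ForwardDetection component, ignoring itself and actors supplied by the game mode's GetFloorMessage.
; A hit while off cooldown calls CastAbility and succeeds; no hit or active cooldown fails the task.
; A failed pawn cast never finishes the task.
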(event EventReceiveExecuteAI
  (params (OwnerController :type AI%20Controller%20Object%20Reference) (ControlledPawn :type Pawn%20Object%20Reference))
  (if (Utilities|IsValid (Variables|Default|GetBaseVehicle))
    _
    (else
      (bind _asbp_wheeled_vehicle_base (Utilities|Casting|CastToBP_WheeledVehicleBase ControlledPawn))
      (Variables|Default|SetBaseVehicle _asbp_wheeled_vehicle_base)))
  (bind _returnvalue (CallFunction|CollisionLineTrace (Variables|/Game/Blueprints/Pawns/BP_WheeledVehicleBase.BP_WheeledVehicleBase_C|GetForwardDetection (Variables|Default|GetBaseVehicle)) 3e+02))
  (if _returnvalue
    (if (Variables|/Game/Blueprints/Pawns/BP_WheeledVehicleBase.BP_WheeledVehicleBase_C|GetbCooldown (Variables|Default|GetBaseVehicle))
      (AI|BehaviorTree|FinishExecute false)
      (else
        (Default|CastAbility (Variables|Default|GetBaseVehicle))
        (AI|BehaviorTree|FinishExecute true)))
    (else
      (AI|BehaviorTree|FinishExecute false))))

(fn CollisionLineTrace
  (params (Target :type Scene%20Component%20Object%20Reference) (Distance :type Float%20%28double-precision%29))
  (bind _returnvalue (Transformation|GetWorldLocation Target))
  (bind _floor (Class|BPIGameMode|GetFloor(Message) (Game|GetGameMode)))
  (LocalVariables|SetNewLocalVar_0 _floor)
  (Utilities|Array|Add (LocalVariables|GetNewLocalVar_0) (Variables|Default|GetBaseVehicle))
  (bind (_outhit _returnvalue_2) (Collision|BoxTraceByChannel _returnvalue (+ (* (Math|Vector|GetForwardVector Target) Distance) _returnvalue) "100.000000,300.000000,400.000000" (Transformation|GetActorRotation (Variables|Default|GetBaseVehicle)) "TraceTypeQuery1" false (LocalVariables|GetNewLocalVar_0) "None"))
  (return _outhit _returnvalue_2))