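; BP_BVTruck is a vehicle Blueprint for a truck that can drop a wall as an ability.
; Pressing the Ability input spawns a BP_WallAbility actor 500 units behind the truck, using the truck's rotation.
; BeginPlay, Tick, overlap and construction logic only call the parent class, so all other behaviour is inherited.
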(event EventBeginPlay
  (|CallParentFunction))

(event Collision|EventActorBeginOverlap
  (params (OtherActor :type Actor%20Object%20Reference))
  (|CallParentFunction OtherActor))

(event EventTick
  (params (DeltaSeconds :type Float%20%28single-precision%29))
  (|CallParentFunction DeltaSeconds))

(event Input|ActionEvents|InputActionAbility
  (params (Key :type Key%20Structure))
  (bind _returnvalue (Transformation|GetActorTransform))
  (:Pressed
    (Game|SpawnActorfromClass "/Game/Blueprints/Abilities/BP_WallAbility.BP_WallAbility_C" (Math|Transform|MakeTransform (+ (.location _returnvalue) (* (Transformation|GetActorForwardVector) -5e+02)) (.rotation _returnvalue) "1,1,1") "Undefined" 0 0)))

(fn ConstructionScript
  (|CallParentFunction))