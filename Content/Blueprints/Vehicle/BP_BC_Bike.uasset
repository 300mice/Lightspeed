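; BP_BC_Bike is a player-controlled bike Blueprint with a blink ability that teleports it forward.
; The Ability input triggers the blink when off cooldown, starting the cooldown and calling HandleSpline before the teleport.
; HandleTeleport disables the controller's moving message, zeroes CharacterMovement velocity and jumps a fixed distance along the forward vector without sweeping.
; After a short delay, the blink re-enables the moving message.
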(event Custom|BlinkAbility
  (if (not (Variables|Default|GetbCooldown))
    (CallFunction|StartCooldown)
    (CallFunction|HandleSpline)
    (|HandleTeleport)
    (Utilities|FlowControl|Delay 0.15)
    (Class|BPIVehicleControls|SetMoving(Message) (Pawn|GetController) true)))

(event EventBeginPlay
  (|CallParentFunction) ; This node is disabled and will not be called.\nDrag off pins to build functionality.
)

(event Collision|EventActorBeginOverlap
  (params (OtherActor :type Actor%20Object%20Reference))
  (|CallParentFunction OtherActor) ; This node is disabled and will not be called.\nDrag off pins to build functionality.
)

(event EventTick
  (params (DeltaSeconds :type Float%20%28single-precision%29))
  (|CallParentFunction DeltaSeconds) ; This node is disabled and will not be called.\nDrag off pins to build functionality.
)

(event Input|ActionEvents|InputActionAbility
  (params (Key :type Key%20Structure :default "None"))
  (:Pressed
    (CallFunction|BlinkAbility)))

(fn ConstructionScript
  (|CallParentFunction))