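; Base vehicle pawn that drives forward constantly, steers with the mouse and leaves a spline trail behind it.
; Tick turns the vehicle by the cursor's horizontal offset from screen center, applied per frame without delta-time scaling.
; BeginPlay spawns a BP_SplineTrail that follows it, with a looping timer adding waypoints.
; Hitting anything not tagged Floor destroys trail and vehicle and clears the controller's moving message.
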(event OnComponentHit(Collider)
  (params (HitComponent :type Primitive%20Component%20Object%20Reference) (OtherActor :type Actor%20Object%20Reference) (OtherComp :type Primitive%20Component%20Object%20Reference) (NormalImpulse :type Vector :default "0, 0, 0") (Hit :type Hit%20Result%20Structure%20%28by%20ref%29))
  (if (not (Actor|ActorHasTag OtherActor "Floor"))
    (Actor|DestroyActor (Variables|Default|GetAs%20BP%20Spline%20Trail))
    (Class|BPIVehicleControls|SetMoving(Message) (Pawn|GetController) false)
    (Actor|DestroyActor)))

(event OnComponentBeginOverlap(Collider)
  (params (OverlappedComponent :type Primitive%20Component%20Object%20Reference) (OtherActor :type Actor%20Object%20Reference) (OtherComp :type Primitive%20Component%20Object%20Reference) (OtherBodyIndex :type Integer) (bFromSweep :type Boolean) (SweepResult :type Hit%20Result%20Structure%20%28by%20ref%29)))

(event Custom|CooldownReset
  (Variables|Default|SetbCooldown false))

(event Custom|StartCooldown
  (Variables|Default|SetbCooldown true)
  (Utilities|Time|SetTimerbyEvent (delegate Custom|CooldownReset) (Variables|Default|GetCooldownTime)))

(event EventBeginPlay
  (Class|BPIVehicleControls|SetMoving(Message) (Game|GetPlayerController (Variables|Default|GetPlayerIndex)) true)
  (CallFunction|HandleSpline))

(event EventTick
  (params (DeltaSeconds :type Float%20%28single-precision%29))
  (Pawn|Input|AddMovementInput (Transformation|GetActorForwardVector) (* 5e+02 (Utilities|Time|GetWorldDeltaSeconds)) true)
  ;[1 1 1] Get Viewport size and divide mouse position by half so that center = 0, left = -0.5, right = 0.5
  (bind _returnvalue (Class|WidgetLayoutLibrary|GetMousePositiononViewport))
  (bind _roundedfloat (CallFunction|RoundtoDecimal (/ (* (.x _returnvalue) (Class|WidgetLayoutLibrary|GetViewportScale)) (.x (Viewport|GetViewportSize))) 1e+01))
  (Class|Actor|AddActorWorldRotation (Math|Rotator|MakeRotator 0.0 0.0 (- _roundedfloat 0.5))))

(fn ConstructionScript)

(fn HandleSpline
  (Utilities|Time|ClearandInvalidateTimerbyHandle (Variables|Default|GetSplineTimer))
  (bind _returnvalue (Game|SpawnActorfromClass "/Game/Blueprints/BP_SplineTrail.BP_SplineTrail_C" (Transformation|GetWorldTransform (Variables|Default|GetSpawnPoint)) "AlwaysSpawn" 0 0))
  (bind _output_get (Variables|Default|SetAs%20BP%20Spline%20Trail _returnvalue))
  (Variables|/Game/Blueprints/BP_SplineTrail.BP_SplineTrail_C|SetFollowVehicle _output_get self)
  (bind _returnvalue_2 (Utilities|Time|SetTimerbyFunctionName (Variables|Default|GetAs%20BP%20Spline%20Trail) "Waypoint Handle" 0.1 true))
  (Variables|Default|SetSplineTimer _returnvalue_2))