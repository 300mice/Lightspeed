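; BP_BC_Car is a car Blueprint that sets its body material according to the current player.
; On BeginPlay it casts the game instance to OnlineGameInstance and switches on CurrentPlayer to apply one of four materials to the mesh's first slot.
; A separate custom event sets a cooldown time and starts audio playback.
; Overlap and Tick are disabled stubs, and the construction script only calls its parent.
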(event Custom|CustomEvent
  (|CallParentFunction)
  (Variables|Default|SetCooldownTime 8.0)
  (Audio|Components|Audio|Play (Variables|Default|GetAudio) 0.0))

(event Collision|EventActorBeginOverlap
  (params (OtherActor :type Actor%20Object%20Reference))
  (|CallParentFunction OtherActor) ; This node is disabled and will not be called.\nDrag off pins to build functionality.
)

(event EventTick
  (params (DeltaSeconds :type Float%20%28single-precision%29))
  (|CallParentFunction DeltaSeconds) ; This node is disabled and will not be called.\nDrag off pins to build functionality.
)

(event EventBeginPlay
  (bind _mesh (Variables|Character|GetMesh))
  (|CallParentFunction)
  (bind _asonline_game_instance (Utilities|Casting|CastToOnlineGameInstance (Game|GetGameInstance)))
  (switch int (Variables|/Game/Multiplayer/OnlineGameInstance.OnlineGameInstance_C|GetCurrentPlayer _asonline_game_instance)
    (:0
      (Rendering|Material|SetMaterial _mesh 0 "/Game/Assets/Enviro/lambert4SG.lambert4SG"))
    (:1
      (Rendering|Material|SetMaterial _mesh 0 "/Game/Assets/Enviro/lambert2SG.lambert2SG"))
    (:2
      (Rendering|Material|SetMaterial _mesh 0 "/Game/Assets/Enviro/lambert3SG.lambert3SG"))
    (:3
      (Rendering|Material|SetMaterial _mesh 0 "/Game/StarterContent/Materials/M_Metal_Gold.M_Metal_Gold"))))

(fn ConstructionScript
  (|CallParentFunction))