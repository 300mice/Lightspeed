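; BP_BVGhostCar is a short-lived ghost car actor, stored with the old vehicle Blueprints.
; On BeginPlay it runs the parent logic, sets the Real flag on its spline trail reference to false and starts its audio.
; It destroys itself after a fixed delay, or earlier when it overlaps any actor not tagged Floor.
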(event EventBeginPlay
  (|CallParentFunction)
  (Variables|/Game/Blueprints/BP_SplineTrail.BP_SplineTrail_C|SetbReal (Variables|Default|GetAs%20BP%20Spline%20Trail) false)
  (Audio|Components|Audio|Play (Variables|Default|GetAudio) 0.0)
  (Utilities|FlowControl|Delay 5.0)
  (Actor|DestroyActor))

(event Collision|EventActorBeginOverlap
  (params (OtherActor :type Actor%20Object%20Reference))
  (|CallParentFunction OtherActor)
  (if (not (Actor|ActorHasTag OtherActor "Floor"))
    (Actor|DestroyActor)))

(event EventTick
  (params (DeltaSeconds :type Float%20%28single-precision%29))
  (|CallParentFunction DeltaSeconds) ; This node is disabled and will not be called.\nDrag off pins to build functionality.
)

(fn ConstructionScript
  (|CallParentFunction))