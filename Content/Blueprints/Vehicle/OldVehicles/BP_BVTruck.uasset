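; BP_BVTruck is a truck vehicle Blueprint, derived from a parent vehicle, whose ability drops a wall behind it.
; On BeginPlay it sets the ability cooldown, starts its audio and picks a mesh material from the ID of player controller 0.
; Pressing the Ability input while off cooldown starts the cooldown and spawns BP_WallAbility at a fixed offset behind the truck, matching its rotation.
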(event EventBeginPlay
  (bind _mesh (Variables|Character|GetMesh))
  (|CallParentFunction)
  (Variables|Default|SetCooldownTime 1e+01)
  (Audio|Components|Audio|Play (Variables|Default|GetAudio) 0.0)
  (switch int (Class|GameplayStatics|GetPlayerControllerID (Game|GetPlayerController 0))
    (:0
      (Rendering|Material|SetMaterial _mesh 0 "/Game/Assets/Enviro/lambert4SG.lambert4SG"))
    (:1
      (Rendering|Material|SetMaterial _mesh 0 "/Game/Assets/Enviro/lambert2SG.lambert2SG"))
    (:2
      (Rendering|Material|SetMaterial _mesh 0 "/Game/Assets/Enviro/lambert3SG.lambert3SG"))
    (:3
      (Rendering|Material|SetMaterial _mesh 0 "/Game/StarterContent/Materials/M_Metal_Gold.M_Metal_Gold"))))

(event Collision|EventActorBeginOverlap
  (params (OtherActor :type Actor%20Object%20Reference))
  (|CallParentFunction OtherActor))

(event EventTick
  (params (DeltaSeconds :type Float%20%28single-precision%29))
  (|CallParentFunction DeltaSeconds))

(event Input|ActionEvents|InputActionAbility
  (params (Key :type Key%20Structure))
  (bind _returnvalue (Transformation|GetActorTransform))
  (:Pressed
    (if (not (Variables|Default|GetbCooldown))
      (CallFunction|StartCooldown)
      (Game|SpawnActorfromClass "/Game/Blueprints/Abilities/BP_WallAbility.BP_WallAbility_C" (Math|Transform|MakeTransform (+ (.location _returnvalue) (* (Transformation|GetActorForwardVector) -5e+02)) (.rotation _returnvalue) "1,1,1") "Undefined" 0 0))))

(fn ConstructionScript
  (|CallParentFunction))