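; BP_BVBike is a player bike vehicle with a cooldown-gated forward teleport ability.
; BeginPlay sets the cooldown time, starts audio and picks the mesh material from the player controller ID.
; The ability input starts the cooldown, calls HandleSpline, then zeroes velocity and jumps the bike forward without a sweep.
; The controller's moving message is switched off for the jump and restored after a short delay.
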(event EventBeginPlay
  (bind _mesh (Variables|Character|GetMesh))
  (|CallParentFunction)
  (Variables|Default|SetCooldownTime 12.0)
  (Audio|Components|Audio|Play (Variables|Default|GetAudio) 0.0)
  (switch int (Class|GameplayStatics|GetPlayerControllerID (Game|GetPlayerController 0))
    (:0
      (Rendering|Material|SetMaterial _mesh 0 "/Game/Assets/Enviro/lambert4SG.lambert4SG"))
    (:1
      (Rendering|Material|SetMaterial _mesh 0 "/Game/Assets/Enviro/lambert2SG.lambert2SG"))
    (:2
      (Rendering|Material|SetMaterial _mesh 0 "/Game/Assets/Enviro/lambert3SG.lambert3SG"))
    (:3
      (Rendering|Material|SetMaterial _mesh 0 "/Game/StarterContent/Materials/M_Metal_Gold.M_Metal_Gold"))))

(event Collision|EventActorBeginOverlap
  (params (OtherActor :type Actor%20Object%20Reference))
  (|CallParentFunction OtherActor))

(event EventTick
  (params (DeltaSeconds :type Float%20%28single-precision%29))
  (|CallParentFunction DeltaSeconds) ; This node is disabled and will not be called.\nDrag off pins to build functionality.
)

(event Input|ActionEvents|InputActionAbility
  (params (Key :type Key%20Structure))
  (:Pressed
    (if (not (Variables|Default|GetbCooldown))
      (CallFunction|StartCooldown)
      (CallFunction|HandleSpline)
      (Utilities|InitiateTeleport)
      (Utilities|FlowControl|Delay 0.15)
      (Class|BPIVehicleControls|SetMoving(Message) (Pawn|GetController) true))))

(fn ConstructionScript
  (|CallParentFunction))