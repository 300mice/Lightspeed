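; Test vehicle character that constantly drives forward, steers by horizontal mouse position and lays a spline trail.
; Each tick forces forward movement input and adds yaw from the rounded, DPI-scaled mouse X centred on the viewport; the yaw is not scaled by delta time.
; On BeginPlay, HandleSpline spawns a BP_SplineTrail at SpawnPoint, set to follow this vehicle, and starts a looping timer on its "Waypoint Handle" function.
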(event EventBeginPlay
  (CallFunction|HandleSpline))

(event Collision|EventActorBeginOverlap
  (params (OtherActor :type Actor%20Object%20Reference)))

(event EventTick
  (params (DeltaSeconds :type Float%20%28single-precision%29))
  (Pawn|Input|AddMovementInput 0 (Transformation|GetActorForwardVector 0) (* 5e+02 (Utilities|Time|GetWorldDeltaSeconds)) true)
  ;[1 1 1] Get Viewport size and divide mouse position by half so that center = 0, left = -0.5, right = 0.5
  (bind _returnvalue (Class|WidgetLayoutLibrary|GetMousePositiononViewport))
  (bind _roundedfloat (CallFunction|RoundtoDecimal (/ (* (.x _returnvalue) (Class|WidgetLayoutLibrary|GetViewportScale)) (.x (Viewport|GetViewportSize))) 1e+01))
  (Class|Actor|AddActorWorldRotation (Math|Rotator|MakeRotator 0.0 0.0 (- _roundedfloat 0.5))))

(fn ConstructionScript)

(fn HandleSpline
  (Utilities|Time|ClearandInvalidateTimerbyHandle (Variables|Default|GetSplineTimer))
  (bind _returnvalue (Game|SpawnActorfromClass "/Game/Blueprints/BP_SplineTrail.BP_SplineTrail_C" (Transformation|GetWorldTransform (Variables|Default|GetSpawnPoint)) "AlwaysSpawn" 0 0))
  (bind _output_get (Variables|Default|SetAs%20BP%20Spline%20Trail _returnvalue))
  (Variables|/Game/Blueprints/BP_SplineTrail.BP_SplineTrail_C|SetFollowVehicle _output_get self)
  (bind _returnvalue_2 (Utilities|Time|SetTimerbyFunctionName (Variables|Default|GetAs%20BP%20Spline%20Trail) "Waypoint Handle" 0.1 true))
  (Variables|Default|SetSplineTimer _returnvalue_2))