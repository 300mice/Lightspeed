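; BP_BVCar is a vehicle Blueprint that adds a ghost ability to the car.
; On Ability input, if not on cooldown, it calls StartCooldown, with the cooldown time set on BeginPlay.
; GhostInitiate spawns a BP_BVGhostCar at the car's transform and swaps the car's mesh material.
; After a fixed delay, GhostEnd sets the material to M_Basic_Wall, leaving the spawned ghost car untouched.
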(event EventBeginPlay
  (|CallParentFunction)
  (Variables|Default|SetCooldownTime 12.0))

(event Collision|EventActorBeginOverlap
  (params (OtherActor :type Actor%20Object%20Reference))
  (|CallParentFunction OtherActor) ; This node is disabled and will not be called.\nDrag off pins to build functionality.
)

(event EventTick
  (params (DeltaSeconds :type Float%20%28single-precision%29))
  (|CallParentFunction DeltaSeconds) ; This node is disabled and will not be called.\nDrag off pins to build functionality.
)

(event Input|ActionEvents|InputActionAbility
  (params (Key :type Key%20Structure :default "None"))
  (:Pressed
    (if (not (Variables|Default|GetbCooldown))
      (CallFunction|StartCooldown)
      (Ghost|GhostInitiate)
      (Utilities|FlowControl|Delay 5.0)
      (Ghost|GhostEnd))))

(fn ConstructionScript
  (|CallParentFunction))

(fn GhostInitiate
  (Game|SpawnActorfromClass "/Game/Blueprints/Vehicle/BP_BVGhostCar.BP_BVGhostCar_C" (Transformation|GetActorTransform) "Undefined" 0 0 0)
  (Rendering|Material|SetMaterial (Variables|Character|GetMesh) 0 "/Game/Assets/Enviro/lambert2SG.lambert2SG"))

(fn GhostEnd
  (Rendering|Material|SetMaterial (Variables|Character|GetMesh) 0 "/Game/StarterContent/Materials/M_Basic_Wall.M_Basic_Wall"))