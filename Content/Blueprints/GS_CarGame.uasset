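; GS_CarGame is the car game's state object, tracking the start countdown, round number and game end.
; GameHasStarted starts a timer that sets RoundPlaying when it fires, while Tick stores its rounded remaining time in CountdownInt.
; IncreaseRound increments CurrentRound on the authority, then calls GameOver, which sets GameEnded at round four.
; HowmanyAlive holds only an unconnected authority switch, and all RepNotify functions are empty.
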(event Custom|IncreaseRound
  (Networking|SwitchHasAuthority
    (:Authority
      (Math|Integer|IncrementInt (Variables|Default|GetCurrentRound)
        (:%20%20
          (CallFunction|GameOver))))))

(event Custom|GameOver
  (Networking|SwitchHasAuthority
    (:Authority
      (if (== (Variables|Default|GetCurrentRound) 4)
        (Variables|Default|SetGameEnded true)))))

(event Custom|HowmanyAlive
  (Networking|SwitchHasAuthority))

(event Custom|StartCountdown
  (Variables|Default|SetRoundPlaying true))

(event Custom|GameHasStarted
  (bind _returnvalue (Utilities|Time|SetTimerbyEvent (delegate Custom|StartCountdown) (Variables|Default|GetTimeToStart)))
  (Variables|Default|SetGameCountdown _returnvalue))

(event EventBeginPlay)

(event EventTick
  (params (DeltaSeconds :type Float%20%28single-precision%29))
  (Variables|Default|SetCountdownInt (Math|Float|Round (Utilities|Time|GetTimerRemainingTimebyHandle (Variables|Default|GetGameCountdown)))))

(fn ConstructionScript)

(fn OnRepCurrentRound)

(fn OnRepGameEnded)

(fn OnRepRoundPlaying)

(fn OnRepPlayersDead)

(fn OnRepCountdownInt)