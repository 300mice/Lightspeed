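; Large arena wall Blueprint that changes colour when its two-players-left event fires and can fade back on a reset event.
; BeginPlay writes a starting white colour to the Wall component's custom primitive data as a vector.
; The ColourChange timeline plays forward for the change, while a separate timeline plays in reverse for the reset.
; Both convert their colour track to sRGB byte channels before writing it each update.
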(event Custom|2PlayersLeft
  (bind _newtrack_0 (Timeline|ColourChange PlayFromStart)
    (:Update
      (Rendering|Material|SetCustomPrimitiveDataVector3 (Variables|Default|GetWall) 0 (Math|Vector|MakeVector (Math|Conversions|ToFloat(Byte) (.R (Math|Color|BreakColor (Math|Conversions|ToColor(LinearColor) _newtrack_0)))) (Math|Conversions|ToFloat(Byte) (.G (Math|Color|BreakColor (Math|Conversions|ToColor(LinearColor) _newtrack_0)))) (Math|Conversions|ToFloat(Byte) (.B (Math|Color|BreakColor (Math|Conversions|ToColor(LinearColor) _newtrack_0)))))))))

(event Custom|ColourReset
  (bind _newtrack_0 (Timeline|Timeline ReverseFromEnd)
    (:Update
      (Rendering|Material|SetCustomPrimitiveDataVector3 (Variables|Default|GetWall) 0 (Math|Vector|MakeVector (Math|Conversions|ToFloat(Byte) (.R (Math|Color|BreakColor (Math|Conversions|ToColor(LinearColor) _newtrack_0)))) (Math|Conversions|ToFloat(Byte) (.G (Math|Color|BreakColor (Math|Conversions|ToColor(LinearColor) _newtrack_0)))) (Math|Conversions|ToFloat(Byte) (.B (Math|Color|BreakColor (Math|Conversions|ToColor(LinearColor) _newtrack_0)))))))))

(event EventBeginPlay
  (bind _whitecolor (Variables|Default|GetWhiteColor))
  (bind (_b _g _r) (Math|Color|BreakColor _whitecolor))
  (Rendering|Material|SetCustomPrimitiveDataVector3 (Variables|Default|GetWall) 0 (Math|Vector|MakeVector (Math|Conversions|ToFloat(Byte) _r) (Math|Conversions|ToFloat(Byte) _g) (Math|Conversions|ToFloat(Byte) _b))))

(fn ConstructionScript)